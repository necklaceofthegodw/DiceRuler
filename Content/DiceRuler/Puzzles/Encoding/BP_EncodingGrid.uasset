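; Grid actor for the Encoding puzzle that spawns and holds a layout of memory pieces.
; CreateGrid derives the piece count from the grid size and offsets a start corner to center the layout on the actor.
; Nested loops step along the parent puzzle fragment's forward and right vectors, spawning BP_MemoryPiece actors, storing them and attaching them to the grid.
; The event graph and construction script are empty.
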(event EventBeginPlay)

(event Collision|EventActorBeginOverlap
  (params (OtherActor :type Actor%20Object%20Reference)))

(event EventTick
  (params (DeltaSeconds :type Float%20%28single-precision%29)))

(fn ConstructionScript)

(fn CreateGrid
  (bind _parentpuzzlefragment (Variables|Default|GetParentPuzzleFragment))
  (bind _fragmentsize (Variables|Default|GetFragmentSize))
  (bind (_x _y) (Math|Vector|BreakVector _fragmentsize))
  (Variables|Default|SetNumberOfPuzzles (* (Variables|Default|GetGridSizeX) (Variables|Default|GetGridSizeY)))
  (Variables|Default|SetInitialPositionOnGrid (- (Transformation|GetActorLocation) (+ (* (Transformation|GetActorRightVector _parentpuzzlefragment) (/ (* _y (- (Variables|Default|GetGridSizeY) 1)) 2.0)) (* (Transformation|GetActorForwardVector _parentpuzzlefragment) (/ (* _x (- (Variables|Default|GetGridSizeX) 1)) 2.0)))))
  (for _index (range 0 (- (Variables|Default|GetGridSizeX) 1))
    (LocalVariables|SetPosOnGrid (+ (Variables|Default|GetInitialPositionOnGrid) (* (Transformation|GetActorForwardVector _parentpuzzlefragment) (* _index (LocalVariables|GetFragmentSizeX)))))
    (for _index_2 (range 0 (- (Variables|Default|GetGridSizeY) 1))
      (bind _returnvalue (Game|SpawnActorfromClass "/Game/DiceRuler/Puzzles/Memory/BP_MemoryPiece.BP_MemoryPiece_C" (Math|Conversions|ToTransform(Vector) (+ (LocalVariables|GetPosOnGrid) (* (Transformation|GetActorRightVector _parentpuzzlefragment) (* _index_2 (LocalVariables|GetFragmentSizeY))))) "Undefined" "MultiplyWithRoot" 0 0 "None" 0))
      (Utilities|Array|Add (Variables|Default|GetSpawnedFragments) _returnvalue)
      (Transformation|AttachActorToActor _returnvalue self "None" "KeepWorld" "KeepWorld" "KeepWorld" true))))