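; Balance scale puzzle actor: fixed toys spawn locked on the second weight, and pickable items are placed on the first.
; Items overlapping Sphere1 snap to the first free socket, tracked in a socket-to-item map, and can be removed again.
; Each change recomputes the second weight mesh's share of both meshes' mass and broadcasts OnWeightChanged.
; The weight-distribution widget receives a reference to the scale on BeginPlay.
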(event OnComponentBeginOverlap(Sphere)
  (params (OverlappedComponent :type Primitive%20Component%20Object%20Reference) (OtherActor :type Actor%20Object%20Reference) (OtherComp :type Primitive%20Component%20Object%20Reference) (OtherBodyIndex :type Integer) (bFromSweep :type Boolean) (SweepResult :type Hit%20Result%20Structure%20%28by%20ref%29))
  ;[1 1 1] adding to the second weight is disabled in this puzzle
)

(event OnComponentBeginOverlap(Sphere1)
  (params (OverlappedComponent :type Primitive%20Component%20Object%20Reference) (OtherActor :type Actor%20Object%20Reference) (OtherComp :type Primitive%20Component%20Object%20Reference) (OtherBodyIndex :type Integer) (bFromSweep :type Boolean) (SweepResult :type Hit%20Result%20Structure%20%28by%20ref%29))
  (bind _asbp_pickable_item (Utilities|Casting|CastToBP_PickableItem OtherActor))
  (CallFunction|AddItemtoSocket _asbp_pickable_item (Variables|Default|GetSM_Weight1)))

(event EventBeginPlay
  (CallFunction|InitWeights)
  (bind _aswbp_weight_distribution (Utilities|Casting|CastToWBP_WeightDistribution (UserInterface|GetUserWidgetObject (Variables|Default|GetWidgetWeightDistribution)))
    (:then
      (Variables|/Game/DiceRuler/Puzzles/BalancingWeights/WBP_WeightDistribution.WBP_WeightDistribution_C|SetParentBalanceScale _aswbp_weight_distribution self))
    (:CastFailed
      _))
  (for _array_element (Transformation|GetAllSocketNames (Variables|Default|GetSM_Weight1))
    (Utilities|Map|Add (Variables|Default|GetSocketsToItems) _array_element 0)))

(event Collision|EventActorBeginOverlap
  (params (OtherActor :type Actor%20Object%20Reference)))

(event EventTick
  (params (DeltaSeconds :type Float%20%28single-precision%29)))

(fn ConstructionScript)

(fn InitWeights
  (bind _sm_weight2 (Variables|Default|GetSM_Weight2))
  (for (_array_element _array_index) (LocalVariables|GetToysToSpawn)
    (bind _returnvalue (Game|SpawnActorfromClass _array_element (Math|Conversions|ToTransform(Vector) (Transformation|GetSocketLocation _sm_weight2 (Utilities|Array|Get(acopy) (Transformation|GetAllSocketNames _sm_weight2) _array_index))) "Undefined" "MultiplyWithRoot" 0 0))
    (Default|DisableInteraction _returnvalue)
    (Transformation|AttachComponentToComponent _returnvalue (Variables|Default|GetSM_Weight2) (Utilities|Array|Get(acopy) (Transformation|GetAllSocketNames _sm_weight2) _array_index) "SnapToTarget" "SnapToTarget" "KeepWorld" true)))

(fn AddItemtoSocket
  (params (Item :type BP%20Pickable%20Item%20Object%20Reference) (WeightMesh :type Scene%20Component%20Object%20Reference))
  (Utilities|IsValid Item
    (:Is%20Valid
      (Variables|/Game/DiceRuler/Gameplay/Pickables/BP_PickableItem.BP_PickableItem_C|SetBalanceScale Item self)
      (bind _socketname (CallFunction|GetFirstEmptySocket))
      (if (not (== _socketname ""))
        (Utilities|Map|Add (Variables|Default|GetSocketsToItems) _socketname Item)
        (Transformation|AttachComponentToComponent Item WeightMesh _socketname "SnapToTarget" "SnapToTarget" "KeepRelative" true)
        (CallFunction|UpdateWeightDistribution)
        (Development|PrintString (Utilities|String|Append "adding item: " (Utilities|GetDisplayName Item)))))))

(fn GetFirstEmptySocket
  (bind _socketstoitems (Variables|Default|GetSocketsToItems))
  (bind _keys (Utilities|Map|Keys _socketstoitems))
  (for _array_element _keys
    (if (.ReturnValue (Utilities|Map|Find _socketstoitems _array_element))
      (Utilities|IsValid (.Value (Utilities|Map|Find _socketstoitems _array_element))
        (:Is%20Not%20Valid
          (return _array_element)))))
  (return "None"))

(fn RemoveItemfromSocket
  (params (Item :type BP%20Pickable%20Item%20Object%20Reference))
  (bind _socketstoitems (Variables|Default|GetSocketsToItems))
  (bind _keys (Utilities|Map|Keys _socketstoitems))
  (for _array_element _keys
    (if (.ReturnValue (Utilities|Map|Find _socketstoitems _array_element))
      (if (== (.Value (Utilities|Map|Find _socketstoitems _array_element)) Item)
        (Utilities|Map|Add _socketstoitems _array_element 0)
        (Transformation|DetachFromActor Item "KeepWorld" "KeepWorld" "KeepWorld")
        (CallFunction|UpdateWeightDistribution)
        (Development|PrintString (Utilities|String|Append "removing item: " (Utilities|GetDisplayName Item)))))))

(fn UpdateWeightDistribution
  (bind _output_get (Variables|Default|SetWeight%20Distribution (/ (Physics|GetMass (Variables|Default|GetSM_Weight2)) (+ (Physics|GetMass (Variables|Default|GetSM_Weight1)) (Physics|GetMass (Variables|Default|GetSM_Weight2))))))
  (Default|CallOnWeightChanged _output_get))