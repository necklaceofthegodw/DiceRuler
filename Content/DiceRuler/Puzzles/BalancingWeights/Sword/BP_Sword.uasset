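; BP_Sword is a sword actor, filed under the balancing weights puzzle, meant to break BP_Destroyable objects on overlap.
; On BeginPlay it binds its begin-overlap event to a handler that calls CrumbleCluster on a BP_Destroyable's Geometry Collection.
; The handler casts OverlappedActor, which is the bound actor itself, rather than OtherActor.
; An impulse and delayed-destroy chain is left unconnected and never runs.
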(event Custom|OnActorBeginOverlap_Event
  (params (OverlappedActor :type Actor%20Object%20Reference) (OtherActor :type Actor%20Object%20Reference))
  (bind _asbp_destroyable (Utilities|Casting|CastToBP_Destroyable OverlappedActor))
  (Class|GeometryCollectionComponent|CrumbleCluster (Variables|/Game/DiceRuler/Puzzles/BalancingWeights/BP_Destroyable.BP_Destroyable_C|GetGeometryCollection _asbp_destroyable)))

(event EventBeginPlay
  (EventDispatchers|BindEventtoOnActorBeginOverlap (delegate Custom|OnActorBeginOverlap_Event)))

(event Collision|EventActorBeginOverlap
  (params (OtherActor :type Actor%20Object%20Reference)))

(event EventTick
  (params (DeltaSeconds :type Float%20%28single-precision%29)))

(fn ConstructionScript)