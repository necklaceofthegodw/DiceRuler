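; Pipes puzzle actor that hosts a pipe minigame and lowers the room's water once it is solved.
; SpawnPuzzle spawns a BP_PipePuzzleManager with a random available level from the map fragment manager and binds to its completion event.
; Triggering switches input mode and blends the view to the manager.
; Finishing restores the player's camera and input, then a timeline sinks the water to just above the new floor.
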(event Custom|SwitchBackToPlayerCamera
  (bind _ns_water (Variables|Default|GetNS_Water))
  (Game|Player|SetViewTargetwithBlend (CallFunction|GetDicePlayerController) (CallFunction|GetDicePlayerCharacter) 0.0 "VTBlend_Linear" 0.0 false)
  (Default|ChangeInputMode (CallFunction|GetDiceRulerGameInstance) "NewEnumerator0")
  ;[1 1 1] Decrease water level after completing puzzle
  (bind _output_get (Variables|Default|SetInitialWaterLocation (Variables|/Script/Engine.SceneComponent|GetRelativeLocation _ns_water)))
  (bind _waterlevel (Timeline|MoveWater Play)
    (:Update
      (Transformation|SetRelativeLocation _ns_water (Math|Vector|MakeVector (.X (Math|Vector|BreakVector _output_get)) (.Y (Math|Vector|BreakVector _output_get)) (Math|Float|Lerp (.Z (Math|Vector|BreakVector _output_get)) (+ (.Z (Math|Vector|BreakVector (Variables|/Script/Engine.SceneComponent|GetRelativeLocation (Variables|Default|GetSM_NewFloor)))) 2e+01) _waterlevel)) false false))))

(event EventBeginPlay
  (|CallParentFunction))

(event Collision|EventActorBeginOverlap
  (params (OtherActor :type Actor%20Object%20Reference))
  (|CallParentFunction OtherActor) ; This node is disabled and will not be called.\nDrag off pins to build functionality.
)

(event EventTick
  (params (DeltaSeconds :type Float%20%28single-precision%29))
  (|CallParentFunction DeltaSeconds) ; This node is disabled and will not be called.\nDrag off pins to build functionality.
)

(fn ConstructionScript
  (|CallParentFunction))

(fn SpawnPuzzle
  (bind _sm_puzzlespawntransform2 (Variables|Default|GetSM_PuzzleSpawnTransform2))
  (bind _returnvalue (Transformation|GetWorldTransform _sm_puzzlespawntransform2))
  (bind (_location _rotation _scale) (Math|Transform|BreakTransform _returnvalue))
  (bind (_roll _pitch _yaw) (Math|Rotator|BreakRotator _rotation))
  (|CallParentFunction)
  (bind _output_get (Variables|Default|SetLevel (Default|GetRandomAvailableLevelPipesPuzzle (CallFunction|GetDiceMapFragmentManager))))
  (bind _returnvalue_2 (Game|SpawnActorfromClass "/Game/DiceRuler/Puzzles/Pipes/BP_PipePuzzleManager.BP_PipePuzzleManager_C" (Math|Transform|MakeTransform _location (Math|Rotator|MakeRotator _roll _pitch (- _yaw (.Yaw (Math|Rotator|BreakRotator (Transformation|GetActorRotation))))) _scale) "Undefined" "MultiplyWithRoot" 0 _output_get 0))
  (bind _output_get_2 (Variables|Default|SetPuzzleManager _returnvalue_2))
  (EventDispatchers|BindEventtoPuzzleCompleted _output_get_2 (EventDispatchers|CreateEvent :!event PuzzleFinished)))

(fn PuzzleFinished
  (|CallParentFunction)
  (CallFunction|SwitchBacktoPlayerCamera))

(fn PuzzleTriggered
  (|CallParentFunction)
  (Default|ChangeInputMode (CallFunction|GetDiceRulerGameInstance) "NewEnumerator3")
  (Game|Player|SetViewTargetwithBlend (CallFunction|GetDicePlayerController) (Variables|Default|GetPuzzleManager) 0.0 "VTBlend_Linear" 0.0 false))