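; Manager for the pipe rotation puzzle, which spawns a square grid of BP_Pipe actors from the level's data table row.
; In Puzzle input mode, Tick highlights the pipe under the cursor via a visibility trace.
; Selecting a pipe rotates it 90 degrees, then compares every yaw against the finished-level table, allowing straight pipes their 180-degree symmetry.
; A full match calls PuzzleCompleted; the camera is offset for 5-wide grids.
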(event EventBeginPlay
  (CallFunction|CreateGrid)
  (EventDispatchers|BindEventtoClickedSomething (CallFunction|GetDicePlayerController) (EventDispatchers|CreateEvent :!event CheckPuzzleClicked)))

(event Collision|EventActorBeginOverlap
  (params (OtherActor :type Actor%20Object%20Reference)))

(event EventTick
  (params (DeltaSeconds :type Float%20%28single-precision%29))
  (switch Utilities|FlowControl|Switch|SwitchonE_InputMode (CallFunction|GetCurrentInputMode)
    (:NewEnumerator3
      (CallFunction|HighlightSelectable (Variables|Default|GetSelectables)))))

(fn ConstructionScript)

(fn CreateGrid
  (bind _level (Variables|Default|GetLevel))
  (bind _fragmentsize (Variables|Default|GetFragmentSize))
  (bind (_x _y) (Math|Vector|BreakVector _fragmentsize))
  (bind _returnvalue (Utilities|GetDataTableRow "/Game/DiceRuler/Puzzles/Pipes/DT_PipesLevels.DT_PipesLevels" _level)
    (:then
      (LocalVariables|SetPipeGridInfo (.PipeGridInfo (Utilities|Struct|BreakS_PipeLevelInfo _returnvalue)))
      (bind _returnvalue_2 (Utilities|GetDataTableRow "/Game/DiceRuler/Puzzles/Pipes/DT_PipesLevelsFinished.DT_PipesLevelsFinished" _level)
        (:then
          (Variables|Default|SetCompletedPipeGridInfo (.PipeGridInfo (Utilities|Struct|BreakS_PipeLevelInfo _returnvalue_2)))
          (Variables|Default|SetGridSizeX (.GridSize (Utilities|Struct|BreakS_PipeLevelInfo _returnvalue)))
          (Variables|Default|SetGridSizeY (.GridSize (Utilities|Struct|BreakS_PipeLevelInfo _returnvalue)))
          (CallFunction|MoveCamera)
          (Variables|Default|SetNumberOfPuzzles (* (Variables|Default|GetGridSizeX) (Variables|Default|GetGridSizeY)))
          (Variables|Default|SetInitialPositionOnGrid (- (Transformation|GetActorLocation) (Math|Vector|MakeVector (/ (* _x (- (Variables|Default|GetGridSizeX) 1)) 2.0) (/ (* _y (- (Variables|Default|GetGridSizeY) 1)) 2.0) 0.0)))
          (for _index (range 0 (- (Variables|Default|GetGridSizeY) 1))
            (LocalVariables|SetPosOnGrid (+ (Variables|Default|GetInitialPositionOnGrid) (Math|Vector|MakeVector 0.0 (* _index (.Y (Math|Vector|BreakVector (Variables|Default|GetFragmentSize)))) 0.0)))
            (for _index_2 (range 0 (- (Variables|Default|GetGridSizeX) 1))
              (bind _returnvalue_3 (Game|SpawnActorfromClass "/Game/DiceRuler/Puzzles/Pipes/BP_Pipe.BP_Pipe_C" (Math|Conversions|ToTransform(Vector) (+ (LocalVariables|GetPosOnGrid) (Math|Vector|MakeVector (* _index_2 (.X (Math|Vector|BreakVector (Variables|Default|GetFragmentSize)))) 0.0 0.0))) "Undefined" "MultiplyWithRoot" 0 (.MeshIndex (Utilities|Struct|BreakS_PipeInfo (Utilities|Array|Get(acopy) (LocalVariables|GetPipeGridInfo) (+ (* _index (Variables|Default|GetGridSizeY)) _index_2)))) (.Rotation (Utilities|Struct|BreakS_PipeInfo (Utilities|Array|Get(acopy) (LocalVariables|GetPipeGridInfo) (+ (* _index (Variables|Default|GetGridSizeY)) _index_2)))) 0 "None" 0))
              (Utilities|Array|Add (Variables|Default|GetSelectables) _returnvalue_3)
              (Transformation|AttachActorToActor _returnvalue_3 self "None" "KeepWorld" "KeepWorld" "KeepWorld" true))))))))

(fn CheckActorUnderCursor
  (bind _returnvalue (Game|GetPlayerController 0))
  (bind (_hitresult _returnvalue_2) (Game|Player|GetHitResultUnderCursorbyChannel _returnvalue "TraceTypeQuery1" true))
  (if _returnvalue_2
    (return (.HitActor (Collision|BreakHitResult _hitresult)))
    (else
      (return 0))))

(fn HighlightSelectable
  (params (Selectables :type Array%20of%20BP%20Selectable%20Object%20Object%20References))
  (bind _actorundercursor (CallFunction|CheckActorUnderCursor))
  (bind _asbp_selectable_object (Utilities|Casting|CastToBP_SelectableObject _actorundercursor)
    (:then
      (if (Utilities|Array|ContainsItem Selectables _asbp_selectable_object)
        (if (== (Variables|Selecting|GetHighlightedSelectable) 0)
          (Default|SetHighlight _asbp_selectable_object "NewEnumerator1")
          (Variables|Selecting|SetHighlightedSelectable _asbp_selectable_object)
          (elif (== (Variables|Selecting|GetHighlightedSelectable) (Variables|Selecting|GetSelectedSelectable))
            (Variables|Selecting|SetHighlightedSelectable 0)
            (elif (not (== _asbp_selectable_object (Variables|Selecting|GetSelectedSelectable)))
              (if (not (== (Variables|Selecting|GetHighlightedSelectable) _asbp_selectable_object))
                (Default|SetHighlight (Variables|Selecting|GetHighlightedSelectable) "NewEnumerator0")
                (Default|SetHighlight _asbp_selectable_object "NewEnumerator1")
                (Variables|Selecting|SetHighlightedSelectable _asbp_selectable_object)))))))
    (:CastFailed
      (Utilities|IsValid (Variables|Selecting|GetHighlightedSelectable)
        (:Is%20Valid
          (if (not (== (Variables|Selecting|GetSelectedSelectable) (Variables|Selecting|GetHighlightedSelectable)))
            (Default|SetHighlight (Variables|Selecting|GetHighlightedSelectable) "NewEnumerator0")
            (Variables|Selecting|SetHighlightedSelectable 0)))))))

(fn SelectSelectable
  (params (Selectables :type Array%20of%20BP%20Selectable%20Object%20Object%20References) (SelectableHit :type BP%20Selectable%20Object%20Object%20Reference))
  (if (Utilities|Array|ContainsItem Selectables SelectableHit)
    ;[1 1 1] Hitting selected more than one time
    (if (== (Variables|Default|GetCurrentlySelected) SelectableHit)
      _
      (else
        (Variables|Default|SetCurrentlySelected SelectableHit)
        (Default|SetSelected (Variables|Default|GetCurrentlySelected) false)))
    (Default|SetSelected SelectableHit true)
    (Transformation|AddActorLocalRotation (Variables|Default|GetCurrentlySelected) "0.000000,90.000000,0.000000" false false)
    (CallFunction|CheckPipesRotation)))

(fn CheckPuzzleClicked
  (bind _actorundercursor (CallFunction|CheckActorUnderCursor))
  (bind _asbp_selectable_object (Utilities|Casting|CastToBP_SelectableObject _actorundercursor))
  (CallFunction|SelectSelectable (Variables|Default|GetSelectables) _asbp_selectable_object))

(fn CheckPipesRotation
  (LocalVariables|SetIsRotationCorrect? true)
  (bind (_array_element _array_index) (Utilities|Array|ForEachLoopwithBreak (Variables|Default|GetSelectables) :!label _label)
    (:LoopBody
      ;[1 1 1] straight pipe - fits two times horizontally and two times vertically
      (if (== (.MeshIndex (Utilities|Struct|BreakS_PipeInfo (Utilities|Array|Get(acopy) (Variables|Default|GetCompletedPipeGridInfo) _array_index))) 1)
        (if (Math|Float|NearlyEqual(Float) (.Yaw (Math|Rotator|BreakRotator (.Rotation (Utilities|Struct|BreakS_PipeInfo (Utilities|Array|Get(acopy) (Variables|Default|GetCompletedPipeGridInfo) _array_index))))) 9e+01 0.1)
          (if (not (or (Math|Float|NearlyEqual(Float) (.Yaw (Math|Rotator|BreakRotator (Transformation|GetActorRotation _array_element))) 9e+01 0.1) (Math|Float|NearlyEqual(Float) (.Yaw (Math|Rotator|BreakRotator (Transformation|GetActorRotation _array_element))) -9e+01 0.1)))
            (LocalVariables|SetIsRotationCorrect? false)
            (goto _label Break))
          (elif (Math|Float|NearlyEqual(Float) (.Yaw (Math|Rotator|BreakRotator (.Rotation (Utilities|Struct|BreakS_PipeInfo (Utilities|Array|Get(acopy) (Variables|Default|GetCompletedPipeGridInfo) _array_index))))) 0.0 0.1)
            (if (not (or (Math|Float|NearlyEqual(Float) (.Yaw (Math|Rotator|BreakRotator (Transformation|GetActorRotation _array_element))) 0.0 0.1) (Math|Float|NearlyEqual(Float) (.Yaw (Math|Rotator|BreakRotator (Transformation|GetActorRotation _array_element))) 1.8e+02 0.1)))
              (LocalVariables|SetIsRotationCorrect? false)
              (goto _label Break))))
        (elif (not (Math|Float|NearlyEqual(Float) (.Yaw (Math|Rotator|BreakRotator (.Rotation (Utilities|Struct|BreakS_PipeInfo (Utilities|Array|Get(acopy) (Variables|Default|GetCompletedPipeGridInfo) _array_index))))) (.Yaw (Math|Rotator|BreakRotator (Transformation|GetActorRotation _array_element))) 0.1))
          (LocalVariables|SetIsRotationCorrect? false)
          (goto _label Break))))
    (:Completed
      (if (LocalVariables|GetIsRotationCorrect?)
        (Default|SetHighlight (Variables|Default|GetCurrentlySelected) "NewEnumerator0")
        (Default|CallPuzzleCompleted)))))

(fn MoveCamera
  (if (== (Variables|Default|GetGridSizeX) 5)
    (Transformation|AddLocalOffset (Variables|Default|GetCamera) (LocalVariables|GetOffset) false false)))