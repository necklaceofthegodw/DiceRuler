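; Pipe piece for the DiceRuler pipes puzzle that sets up its appearance when play begins.
; MeshIndex selects both the static mesh from Meshes and a matching corrective transform from Transforms.
; The actor keeps its location, combines that transform's rotation with StartRotation and multiplies its scale by a fixed uniform factor.
; The construction script only calls its parent, so this setup does not run in the editor preview.
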(event EventBeginPlay
  (bind _meshindex (Variables|Default|GetMeshIndex))
  (bind _transforms (Variables|Default|GetTransforms))
  (bind _output (Utilities|Array|Get(acopy) _transforms _meshindex))
  (bind (_location _rotation _scale) (Math|Transform|BreakTransform _output))
  (|CallParentFunction)
  (Components|StaticMesh|SetStaticMesh (Variables|Default|GetSM_Mesh) (Utilities|Array|Get(acopy) (Variables|Default|GetMeshes) _meshindex))
  (Transformation|SetActorTransform (Math|Transform|MakeTransform (Transformation|GetActorLocation) (Math|Rotator|CombineRotators _rotation (Variables|Default|GetStartRotation)) (* _scale "2.800000,2.800000,2.800000"))))

(event Collision|EventActorBeginOverlap
  (params (OtherActor :type Actor%20Object%20Reference))
  (|CallParentFunction OtherActor) ; This node is disabled and will not be called.\nDrag off pins to build functionality.
)

(event EventTick
  (params (DeltaSeconds :type Float%20%28single-precision%29))
  (|CallParentFunction DeltaSeconds) ; This node is disabled and will not be called.\nDrag off pins to build functionality.
)

(fn ConstructionScript
  (|CallParentFunction))