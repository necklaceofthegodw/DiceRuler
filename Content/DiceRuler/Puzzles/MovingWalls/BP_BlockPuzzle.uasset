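; Lever-and-wall puzzle actor that spawns three levers and four moving walls at component markers on BeginPlay.
; Each lever index flags a fixed, overlapping subset of walls and flips each destination between two Y positions taken from the first two wall markers.
; A shared timeline lerps all flagged walls together, guarded against restarting mid-move, and clears their flags when finished.
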(event Custom|SetWallDestination
  (params (WallIndex :type Integer))
  ;[1 1 1 1 70] Set active wall and it's destination
  (bind _output_get (Variables|Default|SetCurrentMovingWall (Utilities|Array|Get(acopy) (Variables|Default|GetMovingWalls) WallIndex)))
  (Variables|/Game/DiceRuler/Puzzles/MovingWalls/BP_MovingWall.BP_MovingWall_C|SetbMoveMe _output_get true)
  (bind _output_get_2 (Variables|Default|SetStartPos (Transformation|GetActorLocation _output_get)))
  (bind _outdestination (CallFunction|SetMovingWallDestination _output_get_2))
  (Variables|Default|SetEndPos _outdestination)
  (Variables|/Game/DiceRuler/Puzzles/MovingWalls/BP_MovingWall.BP_MovingWall_C|SetStartPos (Variables|Default|GetCurrentMovingWall) (Variables|Default|GetStartPos))
  (Variables|/Game/DiceRuler/Puzzles/MovingWalls/BP_MovingWall.BP_MovingWall_C|SetEndPos (Variables|Default|GetCurrentMovingWall) (Variables|Default|GetEndPos))
  (Utilities|Array|SetArrayElem (Variables|Default|GetMovingWalls) WallIndex (Variables|Default|GetCurrentMovingWall)))

(event Custom|MoveWallsDependingOnLever
  (params (LeverIndex :type Integer))
  ;[1 1 1 1 70] Move some of the walls when activating lever
  (switch int LeverIndex
    (:0
      (CallFunction|SetWallDestination)
      (CallFunction|SetWallDestination 3))
    (:1
      (CallFunction|SetWallDestination)
      (CallFunction|SetWallDestination 1)
      (CallFunction|SetWallDestination 2))
    (:2
      (CallFunction|SetWallDestination 1)
      (CallFunction|SetWallDestination 2)))
  (CallFunction|MoveWalls))

(event Custom|MoveWalls
  ;[1 1 1 1 70] Move all active walls timeline
  (if (not (Variables|Default|GetIsMovingWalls))
    (Variables|Default|SetIsMovingWalls true)
    (bind _distance (Timeline|MoveWallTimeline PlayFromStart)
      (:Update
        (for _array_element (Variables|Default|GetMovingWalls)
          (if (Variables|/Game/DiceRuler/Puzzles/MovingWalls/BP_MovingWall.BP_MovingWall_C|GetbMoveMe _array_element)
            (Transformation|SetActorLocation _array_element (Math|Vector|Lerp(Vector) (Variables|/Game/DiceRuler/Puzzles/MovingWalls/BP_MovingWall.BP_MovingWall_C|GetStartPos _array_element) (Variables|/Game/DiceRuler/Puzzles/MovingWalls/BP_MovingWall.BP_MovingWall_C|GetEndPos _array_element) _distance) false false))))
      (:Finished
        (Variables|Default|SetIsMovingWalls false)
        (for _array_element_2 (Variables|Default|GetMovingWalls)
          (Variables|/Game/DiceRuler/Puzzles/MovingWalls/BP_MovingWall.BP_MovingWall_C|SetbMoveMe _array_element_2 false))))))

(event EventBeginPlay
  ;[1 1 1 1 70] Spawn walls and levers
  (|CallParentFunction)
  (CallFunction|SpawnWallsandLevers))

(event Collision|EventActorBeginOverlap
  (params (OtherActor :type Actor%20Object%20Reference))
  (|CallParentFunction OtherActor) ; This node is disabled and will not be called.\nDrag off pins to build functionality.
)

(event EventTick
  (params (DeltaSeconds :type Float%20%28single-precision%29))
  (|CallParentFunction DeltaSeconds) ; This node is disabled and will not be called.\nDrag off pins to build functionality.
)

(fn ConstructionScript
  (|CallParentFunction))

(fn SpawnWallsandLevers
  (Variables|Default|SetMovingWallsSpawnPlaces (Utilities|Array|MakeArray (Variables|Default|GetSpawn_MovingWall1) (Variables|Default|GetSpawn_MovingWall2) (Variables|Default|GetSpawn_MovingWall3) (Variables|Default|GetSpawn_MovingWall4)))
  (for (_array_element _array_index) (Utilities|Array|MakeArray (Variables|Default|GetSpawnLever1) (Variables|Default|GetSpawnLever2) (Variables|Default|GetSpawnLever3))
    (bind _returnvalue (Game|SpawnActorfromClass "/Game/DiceRuler/Puzzles/MovingWalls/BP_Lever.BP_Lever_C" (Transformation|GetWorldTransform _array_element) "Undefined" "MultiplyWithRoot" 0 _array_index 0 "None" 0))
    (Transformation|AttachActorToActor _returnvalue self "None" "KeepWorld" "KeepWorld" "KeepWorld" true)
    (EventDispatchers|BindEventtoLeverPushed _returnvalue (EventDispatchers|CreateEvent :!event Custom|MoveWallsDependingOnLever)))
  (Variables|Default|SetStartingWallPosY (.Y (Math|Vector|BreakVector (Transformation|GetWorldLocation (Variables|Default|GetSpawn_MovingWall1)))))
  (Variables|Default|SetEndingWallPosY (.Y (Math|Vector|BreakVector (Transformation|GetWorldLocation (Variables|Default|GetSpawn_MovingWall2)))))
  (Utilities|Array|Clear (Variables|Default|GetMovingWalls))
  (for _array_element_2 (Variables|Default|GetMovingWallsSpawnPlaces)
    (bind _returnvalue_2 (Game|SpawnActorfromClass "/Game/DiceRuler/Puzzles/MovingWalls/BP_MovingWall.BP_MovingWall_C" (Transformation|GetWorldTransform _array_element_2) "Undefined" "MultiplyWithRoot" 0 0))
    (Utilities|Array|Add (Variables|Default|GetMovingWalls) _returnvalue_2)
    (bind _output_get (Variables|/Game/DiceRuler/Puzzles/MovingWalls/BP_MovingWall.BP_MovingWall_C|SetStartPos _returnvalue_2 (Math|Vector|MakeVector (.X (Math|Vector|BreakVector (Transformation|GetWorldLocation _array_element_2))) (.Y (Math|Vector|BreakVector (Transformation|GetWorldLocation _array_element_2))) (.Z (Math|Vector|BreakVector (Transformation|GetWorldLocation _array_element_2))))))
    (bind _outdestination (CallFunction|SetMovingWallDestination _output_get))
    (Variables|/Game/DiceRuler/Puzzles/MovingWalls/BP_MovingWall.BP_MovingWall_C|SetEndPos _returnvalue_2 _outdestination)))

(fn SetMovingWallDestination
  (params (CurrentPosition :type Vector))
  (bind (_x _y _z) (Math|Vector|BreakVector CurrentPosition))
  (if (Math|Float|NearlyEqual(Float) _y (Variables|Default|GetEndingWallPosY) 2.0)
    (LocalVariables|SetPosY (Variables|Default|GetStartingWallPosY))
    (else
      (LocalVariables|SetPosY (Variables|Default|GetEndingWallPosY))))
  (return (Math|Vector|MakeVector _x (LocalVariables|GetPosY) _z)))