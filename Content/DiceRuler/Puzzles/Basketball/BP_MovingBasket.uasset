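; BP_MovingBasket is the basket in the Basketball puzzle that detects when enough apples are inside it.
; From BeginPlay, a looping half-second delay polls the TriggerPuzzleComplete volume for overlapping BP_Apple actors instead of relying on overlap events.
; Once the count reaches RequiredPickablesNum, it sets IsBasketFull and calls BasketFull a single time, while the polling keeps running.
; The graphs shown contain no movement logic.
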(event EventBeginPlay
  (CallFunction|CheckBasketTrigger :!label _label)
  (Utilities|FlowControl|Delay 0.5)
  (goto _label))

(event Collision|EventActorBeginOverlap
  (params (OtherActor :type Actor%20Object%20Reference)))

(event EventTick
  (params (DeltaSeconds :type Float%20%28single-precision%29)))

(fn ConstructionScript)

(fn CheckBasketTrigger
  (if (and (>= (Utilities|Array|Length (Collision|GetOverlappingActors (Variables|Default|GetTriggerPuzzleComplete) "/Game/DiceRuler/Gameplay/Pickables/BP_Apple.BP_Apple_C" :!class /Script/Engine.PrimitiveComponent)) (Variables|Default|GetRequiredPickablesNum)) (not (Variables|Default|GetIsBasketFull)))
    (Variables|Default|SetIsBasketFull true)
    (Default|CallBasketFull)))