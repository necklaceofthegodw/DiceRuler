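; Basketball puzzle actor that spawns a moving basket and keeps a supply of apples in play, presumably to be thrown into it.
; Two chained timelines lerp the basket through three marker points, then reverse the point array and restart to ping-pong endlessly.
; Tick spawns apples at a random sideways offset from the spawn marker while under the count cap, and each apple's out-of-bounds event decrements that count.
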(event Custom|PickableOutOfBounds
  (Math|Integer|DecrementInt (Variables|Default|GetAppleCount)
    (:%20%20
      (Development|PrintString "apple ooutuuut"))))

(event EventBeginPlay
  (|CallParentFunction)
  (bind _returnvalue (Game|SpawnActorfromClass "/Game/DiceRuler/Puzzles/Basketball/BP_MovingBasket.BP_MovingBasket_C" (Transformation|GetWorldTransform (Variables|Default|GetSM_BasketPoint1)) "Undefined" "MultiplyWithRoot" 0 0))
  (Variables|Default|SetMovingBasket _returnvalue)
  (Variables|Default|SetPoints (Utilities|Array|MakeArray (Transformation|GetWorldLocation (Variables|Default|GetSM_BasketPoint1)) (Transformation|GetWorldLocation (Variables|Default|GetSM_BasketPoint2)) (Transformation|GetWorldLocation (Variables|Default|GetSM_BasketPoint3))))
  (bind _positionx (Timeline|MoveBasket PlayFromStart)
    (:Update
      (Transformation|SetActorLocation (Variables|Default|GetMovingBasket) (Math|Vector|Lerp(Vector) (Utilities|Array|Get(acopy) (Variables|Default|GetPoints)) (Utilities|Array|Get(acopy) (Variables|Default|GetPoints) 1) _positionx) false false))
    (:Finished
      (bind _positionx_2 (Timeline|MoveBasket2 PlayFromStart)
        (:Update
          (Transformation|SetActorLocation (Variables|Default|GetMovingBasket) (Math|Vector|Lerp(Vector) (Utilities|Array|Get(acopy) (Variables|Default|GetPoints) 1) (Utilities|Array|Get(acopy) (Variables|Default|GetPoints) 2) _positionx_2) false false))
        (:Finished
          (Utilities|Array|Reverse (Variables|Default|GetPoints))
          (Timeline|MoveBasket PlayFromStart))))))

(event Collision|EventActorBeginOverlap
  (params (OtherActor :type Actor%20Object%20Reference))
  (|CallParentFunction OtherActor) ; This node is disabled and will not be called.\nDrag off pins to build functionality.
)

(event EventTick
  (params (DeltaSeconds :type Float%20%28single-precision%29))
  (|CallParentFunction DeltaSeconds)
  (if (< (Variables|Default|GetAppleCount) 5)
    (bind _returnvalue (Game|SpawnActorfromClass "/Game/DiceRuler/Gameplay/Pickables/BP_Apple.BP_Apple_C" (Math|Conversions|ToTransform(Vector) (+ (Transformation|GetWorldLocation (Variables|Default|GetSM_AppleSpawn)) (* (Transformation|GetActorRightVector) (Math|Random|RandomFloatinRange -3e+02 3e+02)))) "Undefined" "MultiplyWithRoot" 0 0))
    (EventDispatchers|BindEventtoPickableOutOfBounds _returnvalue (EventDispatchers|CreateEvent :!event Custom|PickableOutOfBounds))
    (Math|Integer|IncrementInt (Variables|Default|GetAppleCount))))

(fn ConstructionScript
  (|CallParentFunction))