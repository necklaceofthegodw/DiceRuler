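; Manager for the basketball puzzle that spawns a moving basket and apples, and reports completion to its parent puzzle.
; On BeginPlay it aligns to the parent's trigger, tilts a plane, then ping-pongs the basket along four markers using timelines.
; Tick spawns apples at random sideways offsets up to slightly above the required count; their out-of-bounds binding is disconnected.
; A full basket finishes the puzzle and reverses the plane tilt.
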(event Custom|BasketFull
  (Default|PuzzleFinished (Variables|Default|GetParentPuzzle))
  (CallFunction|RotatePlane true))

(event Custom|RotatePlane
  (params (Reverse :type Boolean))
  (if Reverse
    (bind _rotation (Timeline|RotatePlaneTimeline ReverseFromEnd)
      (:Update
        (Transformation|SetRelativeRotation (Variables|Default|GetSM_Plane) (Math|Rotator|MakeRotator 0.0 (Math|Float|Lerp 0.0 15.0 _rotation) 0.0) false false))
      (:Finished
        (if (not Reverse)
          (CallFunction|MoveBasket))))
    (else
      (Timeline|RotatePlaneTimeline PlayFromStart))))

(event Custom|PickableOutOfBounds
  (Math|Integer|DecrementInt (Variables|Default|GetAppleCount)
    (:%20%20
      (Development|PrintString "pickable out of bounds"))))

(event Custom|MoveBasket
  ;[1 1 1] Move basket between positions in Points array
  (bind _positionx (Timeline|Timeline PlayFromStart)
    (:Update
      (Transformation|SetActorLocation (Variables|Default|GetMovingBasket) (Math|Vector|Lerp(Vector) (Utilities|Array|Get(acopy) (Variables|Default|GetPoints) (Variables|Default|GetCnt)) (Utilities|Array|Get(acopy) (Variables|Default|GetPoints) (+ (Variables|Default|GetCnt) 1)) _positionx) false false))
    (:Finished
      (Math|Integer|IncrementInt (Variables|Default|GetCnt)
        (:%20%20
          (if (== (Variables|Default|GetCnt) (- (Utilities|Array|Length (Variables|Default|GetPoints)) 1))
            (Variables|Default|SetCnt 0)
            (Utilities|Array|Reverse (Variables|Default|GetPoints))
            (Timeline|Timeline PlayFromStart)
            (elif (not (Variables|/Game/DiceRuler/MapGeneration/Blueprints/BP_PuzzleMapFragment.BP_PuzzleMapFragment_C|GetPuzzleFinished? (Variables|Default|GetParentPuzzle)))
              (Timeline|Timeline PlayFromStart))))))))

(event EventBeginPlay
  (CallFunction|SetRotationtoParent)
  (bind _returnvalue (Game|SpawnActorfromClass "/Game/DiceRuler/Puzzles/Basketball/BP_MovingBasket.BP_MovingBasket_C" (Transformation|GetWorldTransform (Variables|Default|GetSM_BasketPoint1)) "Undefined" "MultiplyWithRoot" 0 (Variables|Default|GetRequired%20PickablesNum) 0))
  (bind _output_get (Variables|Default|SetMovingBasket _returnvalue))
  (EventDispatchers|BindEventtoBasketFull _output_get (EventDispatchers|CreateEvent :!event Custom|BasketFull))
  (Variables|Default|SetPoints (Utilities|Array|MakeArray (Transformation|GetWorldLocation (Variables|Default|GetSM_BasketPoint1)) (Transformation|GetWorldLocation (Variables|Default|GetSM_BasketPoint2)) (Transformation|GetWorldLocation (Variables|Default|GetSM_BasketPoint3)) (Transformation|GetWorldLocation (Variables|Default|GetSM_BasketPoint4))))
  (CallFunction|RotatePlane false))

(event Collision|EventActorBeginOverlap
  (params (OtherActor :type Actor%20Object%20Reference)))

(event EventTick
  (params (DeltaSeconds :type Float%20%28single-precision%29))
  (if (not (Variables|/Game/DiceRuler/MapGeneration/Blueprints/BP_PuzzleMapFragment.BP_PuzzleMapFragment_C|GetPuzzleFinished? (Variables|Default|GetParentPuzzle)))
    (if (< (Variables|Default|GetAppleCount) (+ (Variables|Default|GetRequired%20PickablesNum) 3))
      (bind _returnvalue (Game|SpawnActorfromClass "/Game/DiceRuler/Gameplay/Pickables/BP_Apple.BP_Apple_C" (Math|Conversions|ToTransform(Vector) (+ (Transformation|GetWorldLocation (Variables|Default|GetSM_AppleSpawn)) (* (Transformation|GetActorRightVector) (Math|Random|RandomFloatinRange -3e+02 3e+02)))) "Undefined" "MultiplyWithRoot" 0 0))
      (Math|Integer|IncrementInt (Variables|Default|GetAppleCount)))))

(fn ConstructionScript)

(fn SetRotationtoParent
  (bind _returnvalue (Transformation|GetActorRotation))
  (bind (_roll _pitch) (Math|Rotator|BreakRotator _returnvalue))
  (Transformation|SetActorRotation (Math|Rotator|MakeRotator _roll _pitch (.Yaw (Math|Rotator|BreakRotator (Transformation|GetWorldRotation (Variables|/Game/DiceRuler/MapGeneration/Blueprints/BP_PuzzleMapFragment.BP_PuzzleMapFragment_C|GetStartPuzzleTrigger2 (Variables|Default|GetParentPuzzle))))))))