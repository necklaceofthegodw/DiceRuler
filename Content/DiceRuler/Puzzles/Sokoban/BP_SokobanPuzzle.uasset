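; Sokoban puzzle actor that manages the lifecycle of a box-pushing puzzle and its HUD menu.
; On spawn, it gets a random available level from the map fragment manager, reads its DT_Sokoban row, and spawns an attached BP_SokobanGrid, binding its finished event.
; Triggering resets the grid and shows the menu.
; Finishing hides the menu, destroys the grid, and teleports the player back to the start trigger after a delay.
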(event Custom|TeleportPlayerBack
  (CallFunction|ShowPuzzleMenu false)
  (Utilities|FlowControl|Delay 2.0)
  (Transformation|SetActorLocation (CallFunction|GetDicePlayerCharacter) (Transformation|GetWorldLocation (Variables|Default|GetStartPuzzleTrigger2)) false true))

(event EventBeginPlay
  (|CallParentFunction))

(event Collision|EventActorBeginOverlap
  (params (OtherActor :type Actor%20Object%20Reference))
  (|CallParentFunction OtherActor) ; This node is disabled and will not be called.\nDrag off pins to build functionality.
)

(event EventTick
  (params (DeltaSeconds :type Float%20%28single-precision%29))
  (|CallParentFunction DeltaSeconds) ; This node is disabled and will not be called.\nDrag off pins to build functionality.
)

(fn ConstructionScript
  (|CallParentFunction))

(fn ResetPuzzle
  (Default|ResetGrid (Variables|Default|GetSokobanGrid)))

(fn SpawnPuzzle
  (|CallParentFunction)
  (bind _output_get (LocalVariables|SetNewLocalVar (Default|GetRandomAvailableLevelSokobanPuzzle (CallFunction|GetDiceMapFragmentManager))))
  (bind _returnvalue (Utilities|GetDataTableRow "/Game/DiceRuler/Puzzles/Sokoban/Data/DT_Sokoban.DT_Sokoban" _output_get)
    (:then
      (bind _output_get_2 (Variables|Default|SetSokobanData _returnvalue))
      (bind _returnvalue_2 (Game|SpawnActorfromClass "/Game/DiceRuler/Puzzles/Sokoban/BP_SokobanGrid.BP_SokobanGrid_C" (Transformation|GetWorldTransform (Variables|Default|GetGridSpawnPoint)) "Undefined" "MultiplyWithRoot" 0 _output_get_2 0))
      (bind _output_get_3 (Variables|Default|SetSokobanGrid _returnvalue_2))
      (Transformation|AttachActorToActor _output_get_3 self "None" "KeepWorld" "KeepWorld" "KeepWorld" true)
      (EventDispatchers|BindEventtoPuzzleFinished (Variables|Default|GetSokobanGrid) (EventDispatchers|CreateEvent :!event PuzzleFinished)))
    (:RowNotFound
      (Development|PrintString "Wrong name of row from DT_Sokoban"))))

(fn ShowPuzzleMenu
  (params (IsShown :type Boolean))
  (Widget|SetVisibility (Variables|/Game/DiceRuler/HUD/WBP_HUD.WBP_HUD_C|GetWBP_Sokoban (Variables|/Game/DiceRuler/HUD/BP_DiceRulerHUD.BP_DiceRulerHUD_C|GetWBP_HUD (CallFunction|GetDiceHud))) (select IsShown "Visible" "Collapsed")))

(fn PuzzleFinished
  (|CallParentFunction)
  (CallFunction|TeleportPlayerBack)
  (CallFunction|DestroyGrid)
  (Development|PrintString "puzzle finished"))

(fn PuzzleTriggered
  (|CallParentFunction)
  (CallFunction|ResetPuzzle)
  (CallFunction|ShowPuzzleMenu true))

(fn DestroyGrid
  (bind _sokobangrid (Variables|Default|GetSokobanGrid))
  (Default|DestroySpawnedActors _sokobangrid)
  (Actor|DestroyActor _sokobangrid))