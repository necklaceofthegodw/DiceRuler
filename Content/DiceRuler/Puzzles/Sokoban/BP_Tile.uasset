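; BP_Tile is a floor tile for the Sokoban puzzle that reports when a pushable box enters or leaves it.
; Its Box collision casts overlapping actors to BP_SimpleBox and fires the OnTileReached dispatcher with an on/off flag, the tile and the box.
; The construction script gives the Plane the target material when IsTargetTile is set, otherwise a translucent one.
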(event OnComponentBeginOverlap(Box)
  (params (OverlappedComponent :type Primitive%20Component%20Object%20Reference) (OtherActor :type Actor%20Object%20Reference) (OtherComp :type Primitive%20Component%20Object%20Reference) (OtherBodyIndex :type Integer) (bFromSweep :type Boolean) (SweepResult :type Hit%20Result%20Structure%20%28by%20ref%29))
  (bind _asbp_simple_box (Utilities|Casting|CastToBP_SimpleBox OtherActor))
  (Default|CallOnTileReached true self _asbp_simple_box))

(event OnComponentEndOverlap(Box)
  (params (OverlappedComponent :type Primitive%20Component%20Object%20Reference) (OtherActor :type Actor%20Object%20Reference) (OtherComp :type Primitive%20Component%20Object%20Reference) (OtherBodyIndex :type Integer))
  (bind _asbp_simple_box (Utilities|Casting|CastToBP_SimpleBox OtherActor))
  (Default|CallOnTileReached false self _asbp_simple_box))

(event EventBeginPlay)

(event Collision|EventActorBeginOverlap
  (params (OtherActor :type Actor%20Object%20Reference)))

(event EventTick
  (params (DeltaSeconds :type Float%20%28single-precision%29)))

(fn ConstructionScript
  (bind _plane (Variables|Default|GetPlane))
  (if (Variables|Default|GetIsTargetTile)
    (Rendering|Material|SetMaterial _plane 0 "/Game/DiceRuler/Puzzles/Sokoban/Textures/M_SokobanTarget.M_SokobanTarget")
    (else
      (Rendering|Material|SetMaterial _plane 0 "/Game/DiceRuler/Puzzles/Sokoban/M_Translucent.M_Translucent"))))