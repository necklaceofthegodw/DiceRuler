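; Sokoban puzzle grid actor that builds a level from a datatable row of character strings.
; BeginPlay scales the plane, creates per-cell trigger boxes and spawns curbs and tiles, recording player and box starts.
; Boxes entering a cell trigger glide to it via timeline, with physics paused.
; ResetGrid teleports the player and spawns or restores boxes; OccupyTile tracks occupancy and fires PuzzleFinished.
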(event Custom|OnBoxOverlapped
  (params (OverlappedComponent :type Primitive%20Component%20Object%20Reference) (OtherActor :type Actor%20Object%20Reference) (OtherComp :type Primitive%20Component%20Object%20Reference) (OtherBodyIndex :type Integer) (bFromSweep :type Boolean) (SweepResult :type Hit%20Result%20Structure%20%28by%20ref%29))
  (if (not (Variables|Default|GetBlockBoxOverlap))
    (bind _asbp_simple_box (Utilities|Casting|CastToBP_SimpleBox OtherActor))
    (Utilities|IsValid (Variables|Default|GetBoxToMove)
      (:Is%20Not%20Valid
        (bind _output_get (Variables|Default|SetBoxToMove _asbp_simple_box))
        (Variables|Default|SetBoxStartLocation (Transformation|GetActorLocation _output_get))
        (Physics|SetSimulatePhysics (Variables|/Game/DiceRuler/Puzzles/Sokoban/BP_SimpleBox.BP_SimpleBox_C|GetCube _output_get) false)
        (bind _position (Timeline|MoveByOne PlayFromStart)
          (:Update
            (Transformation|SetActorLocation (Variables|Default|GetBoxToMove) (Math|Vector|Lerp(Vector) (Variables|Default|GetBoxStartLocation) (+ (Transformation|GetWorldLocation OverlappedComponent) "0.000000,0.000000,50.000000") _position) false false))
          (:Finished
            (Physics|SetSimulatePhysics (Variables|/Game/DiceRuler/Puzzles/Sokoban/BP_SimpleBox.BP_SimpleBox_C|GetCube (Variables|Default|GetBoxToMove)) true)
            (Variables|Default|SetBoxToMove 0)))))))

(event EventBeginPlay
  (bind _griddescription (Variables|Default|GetGridDescription))
  (bind _returnvalue (Utilities|Array|Length _griddescription))
  (CallFunction|InitGridDescriptionfromDatatableRow (Variables|Default|GetSokobanRow))
  (if (> _returnvalue 0)
    (Variables|Default|SetCols (Math|Conversions|ToFloat(Integer) (Utilities|String|Len (Utilities|Array|Get(acopy) _griddescription))))
    (Variables|Default|SetRows (Math|Conversions|ToFloat(Integer) _returnvalue))
    (CallFunction|InitGridScaleandTiles)
    (CallFunction|InitBoxCollisions)
    (CallFunction|InitObjectsonGrid)
    (else
      (Development|PrintString "add sokoban grid description"))))

(event Collision|EventActorBeginOverlap
  (params (OtherActor :type Actor%20Object%20Reference)))

(event EventTick
  (params (DeltaSeconds :type Float%20%28single-precision%29)))

(fn ConstructionScript)

(fn InitGridScaleandTiles
  (bind _plane (Variables|Default|GetPlane))
  (bind _returnvalue (Transformation|GetWorldScale _plane))
  (bind (_x _y _z) (Math|Vector|BreakVector _returnvalue))
  (Transformation|SetWorldScale3D _plane (Math|Vector|MakeVector (* _x (/ (Variables|Default|GetRows) 4.0)) (* _y (/ (Variables|Default|GetCols) 4.0)) _z))
  (Rendering|Material|SetScalarParameterValueonMaterials _plane "GridSizeX" (Variables|Default|GetRows))
  (Rendering|Material|SetScalarParameterValueonMaterials _plane "GridSizeY" (Variables|Default|GetCols)))

(fn InitBoxCollisions
  (bind _tilewidth (LocalVariables|GetTileWidth))
  (bind _returnvalue (/ _tilewidth 2.0))
  (LocalVariables|SetStartPosition (+ (* (Math|Vector|MakeVector (* (/ (Variables|Default|GetRows) 2.0) -1.0) (/ (Variables|Default|GetCols) 2.0) 0.0) (LocalVariables|GetTileWidth)) (Math|Vector|MakeVector _returnvalue (* _returnvalue -1.0) 0.0)))
  (Utilities|Array|Clear (Variables|Default|GetTilePositions))
  (for _index (range 0 (- (Math|Float|Truncate (Variables|Default|GetRows)) 1))
    (for _index_2 (range 0 (- (Math|Float|Truncate (Variables|Default|GetCols)) 1))
      (Utilities|Array|Add (Variables|Default|GetTilePositions) (+ (+ (LocalVariables|GetStartPosition) (Math|Vector|MakeVector (* _index (LocalVariables|GetTileWidth)) (* (* _index_2 (LocalVariables|GetTileWidth)) -1.0) 0.0)) (LocalVariables|GetZOffset)))
      (bind _returnvalue_2 (AddComponent|AddBoxComponent true (Math|Transform|MakeTransform (+ (LocalVariables|GetStartPosition) (Math|Vector|MakeVector (* _index (LocalVariables|GetTileWidth)) (* (* _index_2 (LocalVariables|GetTileWidth)) -1.0) 0.0)))))
      (Components|Box|SetBoxExtent _returnvalue_2 "45.000000,45.000000,45.000000" true)
      (Transformation|AttachComponentToComponent _returnvalue_2 (Variables|Default|GetDefaultSceneRoot) "None" "KeepRelative" "KeepRelative" "KeepRelative" true)
      (Collision|BindEventtoOnComponentBeginOverlap _returnvalue_2 (EventDispatchers|CreateEvent :!event Custom|OnBoxOverlapped)))))

(fn InitObjectsonGrid
  (Utilities|Array|Clear (Variables|Default|GetSpawnedBoxes))
  (Utilities|Array|Clear (Variables|Default|GetBoxesStartPoints))
  (for (_array_element _array_index) (Variables|Default|GetGridDescription)
    (for (_array_element_2 _array_index_2) (Utilities|String|GetCharacterArrayfromString _array_element)
      (LocalVariables|SetCurrentTilePosition (- (Utilities|Array|Get(acopy) (Variables|Default|GetTilePositions) (+ _array_index_2 (* _array_index (Utilities|Array|Length (Utilities|String|GetCharacterArrayfromString _array_element))))) "0.000000,0.000000,100.000000"))
      (switch string _array_element_2
        (:w
          (bind _returnvalue (Game|SpawnActorfromClass "/Game/DiceRuler/Puzzles/Sokoban/BP_Curb.BP_Curb_C" (Math|Conversions|ToTransform(Vector) (+ (LocalVariables|GetCurrentTilePosition) "0.000000,0.000000,20.000000")) "Undefined" "MultiplyWithRoot" 0 0))
          (Transformation|AttachComponentToComponent _returnvalue (Variables|Default|GetDefaultSceneRoot) "None" "KeepRelative" "KeepRelative" "KeepRelative" true))
        (:e
          (bind _returnvalue_2 (Game|SpawnActorfromClass "/Game/DiceRuler/Puzzles/Sokoban/BP_Tile.BP_Tile_C" (Math|Conversions|ToTransform(Vector) (LocalVariables|GetCurrentTilePosition)) "Undefined" "MultiplyWithRoot" 0 false 0))
          (Transformation|AttachComponentToComponent _returnvalue_2 (Variables|Default|GetDefaultSceneRoot) "None" "KeepRelative" "KeepRelative" "KeepRelative" true))
        (:p
          (Variables|Default|SetPlayerStartPoint (Math|Transform|TransformLocation (Transformation|GetActorTransform) (+ (LocalVariables|GetCurrentTilePosition) "0.000000,0.000000,50.000000"))))
        (:b
          (Utilities|Array|Add (Variables|Default|GetBoxesStartPoints) (Math|Transform|TransformLocation (Transformation|GetActorTransform) (+ (LocalVariables|GetCurrentTilePosition) "0.000000,0.000000,50.000000"))))
        (:t
          (bind _returnvalue_3 (Game|SpawnActorfromClass "/Game/DiceRuler/Puzzles/Sokoban/BP_Tile.BP_Tile_C" (Math|Conversions|ToTransform(Vector) (LocalVariables|GetCurrentTilePosition)) "Undefined" "MultiplyWithRoot" 0 true 0))
          (Transformation|AttachComponentToComponent _returnvalue_3 (Variables|Default|GetDefaultSceneRoot) "None" "KeepRelative" "KeepRelative" "KeepRelative" true)
          (EventDispatchers|BindEventtoOnTileReached _returnvalue_3 (EventDispatchers|CreateEvent :!event OccupyTile)))))))

(fn ResetGrid
  (bind _spawnedboxes (Variables|Default|GetSpawnedBoxes))
  (Variables|Default|SetBlockBoxOverlap true)
  (Transformation|SetActorLocation (CallFunction|GetDicePlayerCharacter) (Variables|Default|GetPlayerStartPoint) false true)
  (if (> (Utilities|Array|Length _spawnedboxes) 0)
    (for _array_element _spawnedboxes
      (Transformation|SetActorLocation _array_element (Variables|/Game/DiceRuler/Puzzles/Sokoban/BP_SimpleBox.BP_SimpleBox_C|GetStartPosition _array_element) false true))
    (else
      (for _array_element_2 (Variables|Default|GetBoxesStartPoints)
        (bind _returnvalue (Game|SpawnActorfromClass "/Game/DiceRuler/Puzzles/Sokoban/BP_SimpleBox.BP_SimpleBox_C" (Math|Conversions|ToTransform(Vector) _array_element_2) "Undefined" "MultiplyWithRoot" 0 _array_element_2 0))
        (Utilities|Array|Add (Variables|Default|GetSpawnedBoxes) _returnvalue))))
  (Variables|Default|SetBlockBoxOverlap false))

(fn OccupyTile
  (params (IsOccupied :type Boolean) (Tile :type BP%20Tile%20Object%20Reference) (Box :type BP%20Simple%20Box%20Object%20Reference))
  (bind _tiletooccupied (Variables|Default|GetTileToOccupied))
  (Utilities|Map|Add (Variables|Default|GetBoxToTile) Box Tile)
  (Utilities|Map|Add _tiletooccupied Tile IsOccupied)
  (bind _keys (Utilities|Map|Keys _tiletooccupied))
  (if (== (Utilities|Map|Length (Variables|Default|GetBoxToTile)) (Utilities|Array|Length (Variables|Default|GetSpawnedBoxes)))
    (for _array_element _keys
      (if (not (.ReturnValue (Utilities|Map|Find (Variables|Default|GetTileToOccupied) _array_element)))
        (LocalVariables|SetIsPuzzleFinished false)))
    (if (LocalVariables|GetIsPuzzleFinished)
      (Development|PrintString "sokoban completed, congratulations")
      (Default|CallPuzzleFinished))))

(fn InitGridDescriptionfromDatatableRow
  (params (SokobanRow :type S%20Sokoban%20Row%20Structure))
  (Variables|Default|SetGridDescription (Utilities|Struct|BreakS_SokobanRow SokobanRow)))