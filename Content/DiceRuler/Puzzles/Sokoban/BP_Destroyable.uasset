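; BP_Destroyable is a breakable box actor for the Sokoban puzzle, built on a Geometry Collection.
; Two seconds after BeginPlay it enables damage from collision, then tints the collection's materials according to its BoxTypeString letter.
; An overlap of its Box component with a BP_Sword destroys the actor after a short delay, while any fracturing is left to the Geometry Collection's collision damage.
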(event OnComponentBeginOverlap(Box)
  (params (OverlappedComponent :type Primitive%20Component%20Object%20Reference) (OtherActor :type Actor%20Object%20Reference) (OtherComp :type Primitive%20Component%20Object%20Reference) (OtherBodyIndex :type Integer) (bFromSweep :type Boolean) (SweepResult :type Hit%20Result%20Structure%20%28by%20ref%29))
  (Utilities|Casting|CastToBP_Sword OtherActor)
  (Utilities|FlowControl|Delay 1.5)
  (Actor|DestroyActor))

(event EventBeginPlay
  (bind _geometrycollection (Variables|Default|GetGeometryCollection))
  (Utilities|FlowControl|Delay 2.0)
  (Class|GeometryCollectionComponent|SetEnableDamagefromCollision (Variables|Default|GetGeometryCollection) true)
  (switch string (Variables|Default|GetBoxTypeString)
    (:w
      (Rendering|Material|SetVectorParameterValueonMaterials _geometrycollection "Color" "1.000000,1.000000,1.000000"))
    (:e
      (Rendering|Material|SetVectorParameterValueonMaterials _geometrycollection "Color" "0.500000,1.000000,1.000000"))
    (:p
      (Rendering|Material|SetVectorParameterValueonMaterials _geometrycollection "Color" "1.000000,0.500000,1.000000"))
    (:f
      (Rendering|Material|SetVectorParameterValueonMaterials _geometrycollection "Color" "0.500000,0.500000,1.000000"))
    (:b
      (Rendering|Material|SetVectorParameterValueonMaterials _geometrycollection "Color" "0.300000,0.700000,1.000000"))
    (:t
      (Rendering|Material|SetVectorParameterValueonMaterials _geometrycollection "Color" "0.700000,0.700000,1.000000"))))

(event Collision|EventActorBeginOverlap
  (params (OtherActor :type Actor%20Object%20Reference)))

(event EventTick
  (params (DeltaSeconds :type Float%20%28single-precision%29)))

(fn ConstructionScript)