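; Crushing ball puzzle Blueprint that extends a parent puzzle class and places an angled platform in the level.
; BeginPlay runs the parent logic, then calls the overridden SpawnPuzzle.
; SpawnPuzzle runs the parent spawn, then spawns a BP_AngledPlatform at the SMMovingFloorSpawn1 component's world transform and stores the reference.
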(event EventBeginPlay
  (|CallParentFunction)
  (CallFunction|SpawnPuzzle))

(event Collision|EventActorBeginOverlap
  (params (OtherActor :type Actor%20Object%20Reference))
  (|CallParentFunction OtherActor) ; This node is disabled and will not be called.\nDrag off pins to build functionality.
)

(event EventTick
  (params (DeltaSeconds :type Float%20%28single-precision%29))
  (|CallParentFunction DeltaSeconds) ; This node is disabled and will not be called.\nDrag off pins to build functionality.
)

(fn ConstructionScript
  (|CallParentFunction))

(fn SpawnPuzzle
  (|CallParentFunction)
  (bind _returnvalue (Game|SpawnActorfromClass "/Game/DiceRuler/Puzzles/CrushingBall/BP_AngledPlatform.BP_AngledPlatform_C" (Transformation|GetWorldTransform (Variables|Default|GetSM_MovingFloorSpawn1)) "Undefined" "MultiplyWithRoot" 0 0))
  (Variables|Default|SetBP_AngledPlatform _returnvalue))