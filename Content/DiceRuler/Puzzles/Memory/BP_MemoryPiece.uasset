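; BP_MemoryPiece is a tile for a memory puzzle that shows or hides its assigned image on a plane.
; SetPuzzleImage stores the texture's name and creates a dynamic material instance on the plane, setting the image texture and rune color parameters.
; SetSelected passes the selection state to RevealPuzzleImage, which toggles the plane's hidden-in-game flag; the parent SetSelected call is left unconnected.
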(event EventBeginPlay)

(event Collision|EventActorBeginOverlap
  (params (OtherActor :type Actor%20Object%20Reference)))

(event EventTick
  (params (DeltaSeconds :type Float%20%28single-precision%29)))

(fn ConstructionScript)

(fn SetPuzzleImage
  (params (Val :type Texture%20Object%20Reference) (ColorVal :type Float%20%28single-precision%29))
  (bind _plane (Variables|Default|GetPlane))
  (Variables|Default|SetImageNameString (Utilities|GetObjectName Val))
  (bind _returnvalue (Rendering|Material|CreateDynamicMaterialInstance _plane 0 (Rendering|Material|GetMaterial _plane 0) "None" :!class /Script/Engine.PrimitiveComponent))
  (Rendering|Material|SetTextureParameterValue _returnvalue "ImageParam" Val)
  (Rendering|Material|SetScalarParameterValue _returnvalue "RuneColor" ColorVal :!class /Script/Engine.MaterialInstanceDynamic))

(fn RevealPuzzleImage
  (params (IsRevealed :type Boolean))
  (Development|SetHiddeninGame (Variables|Default|GetPlane) (not IsRevealed) false))

(fn SetSelected
  (params (IsSelected :type Boolean))
  (CallFunction|RevealPuzzleImage IsSelected))