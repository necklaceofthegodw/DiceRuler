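; BP_MemoryPuzzle is a world puzzle actor that hosts a grid-based memory puzzle and hands the player over to it.
; Its SpawnPuzzle override creates a BP_MemoryPuzzleManager at a marker transform, offset by actor yaw, passing grid size and binding its completion event.
; The first player overlap with the start trigger registers the active puzzle, changes input mode and blends the view to the manager.
; SwitchBackToPlayerCamera returns view and input mode to the player.
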(event OnComponentBeginOverlap(StartPuzzleTrigger)
  (params (OverlappedComponent :type Primitive%20Component%20Object%20Reference) (OtherActor :type Actor%20Object%20Reference) (OtherComp :type Primitive%20Component%20Object%20Reference) (OtherBodyIndex :type Integer) (bFromSweep :type Boolean) (SweepResult :type Hit%20Result%20Structure%20%28by%20ref%29))
  (bind _asbp_dice_player_character (Utilities|Casting|CastToBP_DicePlayerCharacter OtherActor))
  (if (not (Variables|Default|GetbPuzzleStarted))
    (Variables|Default|SetbPuzzleStarted true)
    (Default|SetActivePuzzle _asbp_dice_player_character self)
    (bind _asbp_dice_player_controller (Utilities|Casting|CastToBP_DicePlayerController (Pawn|GetController _asbp_dice_player_character)))
    (Default|ChangeInputMode (CallFunction|GetDiceRulerGameInstance) "NewEnumerator3")
    (Game|Player|SetViewTargetwithBlend _asbp_dice_player_controller (Variables|Default|GetPuzzleManager) 0.0 "VTBlend_Linear" 0.0 false)))

(event Custom|SwitchBackToPlayerCamera
  (Game|Player|SetViewTargetwithBlend (CallFunction|GetDicePlayerController) (CallFunction|GetDicePlayerCharacter) 0.0 "VTBlend_Linear" 0.0 false)
  (Default|ChangeInputMode (CallFunction|GetDiceRulerGameInstance) "NewEnumerator0"))

(event EventBeginPlay
  (|CallParentFunction))

(event Collision|EventActorBeginOverlap
  (params (OtherActor :type Actor%20Object%20Reference))
  (|CallParentFunction OtherActor) ; This node is disabled and will not be called.\nDrag off pins to build functionality.
)

(event EventTick
  (params (DeltaSeconds :type Float%20%28single-precision%29))
  (|CallParentFunction DeltaSeconds) ; This node is disabled and will not be called.\nDrag off pins to build functionality.
)

(fn ConstructionScript
  (|CallParentFunction))

(fn SpawnPuzzle
  (bind _sm_puzzlespawntransform (Variables|Default|GetSM_PuzzleSpawnTransform))
  (bind _returnvalue (Transformation|GetWorldTransform _sm_puzzlespawntransform))
  (bind (_location _rotation _scale) (Math|Transform|BreakTransform _returnvalue))
  (bind (_roll _pitch _yaw) (Math|Rotator|BreakRotator _rotation))
  (|CallParentFunction)
  (bind _returnvalue_2 (Game|SpawnActorfromClass "/Game/DiceRuler/Puzzles/Memory/BP_MemoryPuzzleManager.BP_MemoryPuzzleManager_C" (Math|Transform|MakeTransform _location (Math|Rotator|MakeRotator _roll _pitch (- _yaw (.Yaw (Math|Rotator|BreakRotator (Transformation|GetActorRotation))))) _scale) "Undefined" "MultiplyWithRoot" 0 true (Variables|Puzzle|GetGrid%20Size%20X) (Variables|Puzzle|GetGrid%20Size%20Y) 0))
  (bind _output_get (Variables|Default|SetPuzzleManager _returnvalue_2))
  (EventDispatchers|BindEventtoPuzzleCompleted _output_get (EventDispatchers|CreateEvent :!event Custom|SwitchBackToPlayerCamera)))