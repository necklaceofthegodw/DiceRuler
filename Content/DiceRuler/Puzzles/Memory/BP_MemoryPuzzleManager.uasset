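; Manager for the memory-matching puzzle in DiceRuler: spawns a grid of pieces where players find matching image pairs.
; On BeginPlay it builds an even-count grid aligned to the parent puzzle fragment, deals paired images randomly and binds controller clicks.
; Tick highlights pieces under the cursor in Puzzle input mode.
; Two selections trigger a delayed name comparison that deselects mismatches, counts moves and mistakes, and completes the puzzle once all pairs match.
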(event EventBeginPlay
  (Variables|Default|SetFragmentImages (Variables|/Game/DiceRuler/BP_DiceRulerGameInstance.BP_DiceRulerGameInstance_C|GetAllFragmentImages (CallFunction|GetDiceRulerGameInstance)))
  (if (Variables|Default|GetbIsRandomGridSize)
    (Variables|Default|SetGridSizeX (Math|Random|RandomIntegerinRange 3 6)))
  (CallFunction|CreateGrid)
  (CallFunction|SetRotationtoParent)
  (CallFunction|AddImagesRandomly)
  (Transformation|AddLocalRotation (Variables|Default|GetCamera) "-80.000000,270.000000,0.000000" false false)
  (EventDispatchers|BindEventtoClickedSomething (CallFunction|GetDicePlayerController) (EventDispatchers|CreateEvent :!event CheckPuzzleClicked)))

(event Collision|EventActorBeginOverlap
  (params (OtherActor :type Actor%20Object%20Reference)))

(event EventTick
  (params (DeltaSeconds :type Float%20%28single-precision%29))
  (switch Utilities|FlowControl|Switch|SwitchonE_InputMode (CallFunction|GetCurrentInputMode)
    (:NewEnumerator3
      (CallFunction|HighlightSelectable (Variables|Default|GetSpawnedFragments)))))

(fn ConstructionScript)

(fn AddImagesRandomly
  (bind _spawnedfragments (Variables|Default|GetSpawnedFragments))
  (bind _indexesunallocated (LocalVariables|GetIndexesUnAllocated))
  (bind _returnvalue (Utilities|Array|Length _spawnedfragments))
  ;[1 1 1] Adjust puzzle images to grid size
  (if (== _returnvalue (* (Utilities|Array|Length (Variables|Default|GetFragmentImages)) 2))
    (LocalVariables|SetFragmentImagesL (Variables|Default|GetFragmentImages))
    (else
      (for _index (range 0 (- (/ _returnvalue 2) 1))
        (Utilities|Array|Add (LocalVariables|GetFragmentImagesL) (Utilities|Array|Get(acopy) (Variables|Default|GetFragmentImages) _index)))))
  (for _index_2 (range 0 (- (Utilities|Array|Length (Variables|Default|GetSpawnedFragments)) 1))
    (Utilities|Array|Add (LocalVariables|GetIndexesUnAllocated) _index_2))
  (for _array_element (Variables|Default|GetFragmentImages)
    ;[1 1 1] pairs
    (LocalVariables|SetColorVal (Math|Random|RandomFloatinRange 0.0 3.0))
    (for _index_3 (range 0 1)
      (bind _output_get (LocalVariables|SetItemToRemove (Utilities|Array|Get(acopy) _indexesunallocated (Math|Random|RandomIntegerinRange 0 (- (Utilities|Array|Length _indexesunallocated) 1)))))
      (Default|SetPuzzleImage (Utilities|Array|Get(acopy) (Variables|Default|GetSpawnedFragments) _output_get) _array_element (LocalVariables|GetColorVal))
      (Utilities|Array|RemoveItem (LocalVariables|GetIndexesUnAllocated) (LocalVariables|GetItemToRemove)))))

(fn CheckPuzzleClicked
  (bind _actorundercursor (CallFunction|CheckActorUnderCursor))
  (bind _asbp_selectable_object (Utilities|Casting|CastToBP_SelectableObject _actorundercursor))
  (CallFunction|SelectSelectable (Variables|Default|GetSpawnedFragments) _asbp_selectable_object))

(fn CheckActorUnderCursor
  (bind _returnvalue (Game|GetPlayerController 0))
  (bind (_hitresult _returnvalue_2) (Game|Player|GetHitResultUnderCursorbyChannel _returnvalue "TraceTypeQuery1" true))
  (if _returnvalue_2
    (return (.HitActor (Collision|BreakHitResult _hitresult)))
    (else
      (return 0))))

(fn HighlightSelectable
  (params (Selectables :type Array%20of%20BP%20Selectable%20Object%20Object%20References))
  (bind _actorundercursor (CallFunction|CheckActorUnderCursor))
  (bind _asbp_selectable_object (Utilities|Casting|CastToBP_SelectableObject _actorundercursor)
    (:then
      (if (Utilities|Array|ContainsItem Selectables _asbp_selectable_object)
        (if (== (Variables|Default|GetHighlightedSelectable) 0)
          (Default|SetHighlight _asbp_selectable_object "NewEnumerator1")
          (Variables|Default|SetHighlightedSelectable _asbp_selectable_object)
          (elif (== (Variables|Default|GetHighlightedSelectable) (Variables|Default|GetSelectedSelectable))
            (Variables|Default|SetHighlightedSelectable 0)
            (elif (not (== _asbp_selectable_object (Variables|Default|GetSelectedSelectable)))
              (if (not (== (Variables|Default|GetHighlightedSelectable) _asbp_selectable_object))
                (Default|SetHighlight (Variables|Default|GetHighlightedSelectable) "NewEnumerator0")
                (Default|SetHighlight _asbp_selectable_object "NewEnumerator1")
                (Variables|Default|SetHighlightedSelectable _asbp_selectable_object)))))))
    (:CastFailed
      (Utilities|IsValid (Variables|Default|GetHighlightedSelectable)
        (:Is%20Valid
          (if (not (== (Variables|Default|GetSelectedSelectable) (Variables|Default|GetHighlightedSelectable)))
            (Default|SetHighlight (Variables|Default|GetHighlightedSelectable) "NewEnumerator0")
            (Variables|Default|SetHighlightedSelectable 0)))))))

(fn SelectSelectable
  (params (Selectables :type Array%20of%20BP%20Selectable%20Object%20Object%20References) (SelectableHit :type BP%20Selectable%20Object%20Object%20Reference))
  (if (Utilities|Array|ContainsItem Selectables SelectableHit)
    ;[1 1 1] Hitting selected more than one time
    (if (not (or (== (Variables|Default|GetFirstSelected) SelectableHit) (== (Variables|Default|GetSecondSelected) SelectableHit)))
      (Utilities|IsValid (Variables|Default|GetFirstSelected)
        (:Is%20Valid
          (Utilities|IsValid (Variables|Default|GetSecondSelected)
            (:Is%20Not%20Valid
              (Variables|Default|SetSecondSelected SelectableHit)
              (Default|SetSelected SelectableHit true)
              (Utilities|Time|SetTimerbyFunctionName 0 "CheckAndUnselectPuzzlesDelayed" 1.0))))
        (:Is%20Not%20Valid
          (Variables|Default|SetFirstSelected SelectableHit)
          (Default|SetSelected SelectableHit true))))))

(fn CheckifPuzzleImagesAretheSame
  (params (Selectable1 :type BP%20Selectable%20Object%20Object%20Reference) (Selectable2 :type BP%20Selectable%20Object%20Object%20Reference))
  (bind _asbp_memory_piece (Utilities|Casting|CastToBP_MemoryPiece Selectable1)
    (:then
      (bind _asbp_memory_piece_2 (Utilities|Casting|CastToBP_MemoryPiece Selectable2)
        (:then
          (return (Utilities|Enum|Equal(Enum) (Variables|/Game/DiceRuler/Puzzles/Memory/BP_MemoryPiece.BP_MemoryPiece_C|GetImageNameString _asbp_memory_piece_2) (Variables|/Game/DiceRuler/Puzzles/Memory/BP_MemoryPiece.BP_MemoryPiece_C|GetImageNameString _asbp_memory_piece))))
        (:CastFailed
          _)))
    (:CastFailed
      _))
  (return false))

(fn CheckandUnselectPuzzlesDelayed
  (bind _outthesame_ (CallFunction|CheckifPuzzleImagesAretheSame (Variables|Default|GetFirstSelected) (Variables|Default|GetSecondSelected)))
  (if _outthesame_
    _
    (else
      (Default|SetSelected (Variables|Default|GetFirstSelected) false)
      (Math|Integer|IncrementInt (Variables|Default|GetMistakesCnt)
        (:%20%20
          _))))
  (Variables|Default|SetFirstSelected 0)
  (Variables|Default|SetSecondSelected 0)
  (Math|Integer|IncrementInt (Variables|Default|GetMovesCnt)
    (:%20%20
      (if (== (- (Variables|Default|GetMovesCnt) (Variables|Default|GetMistakesCnt)) (/ (Variables|Default|GetNumberOfPuzzles) 2))
        (Default|CallPuzzleCompleted)))))

(fn SetRotationtoParent
  (bind _returnvalue (Transformation|GetActorRotation))
  (bind (_roll _pitch) (Math|Rotator|BreakRotator _returnvalue))
  (Transformation|SetActorRotation (Math|Rotator|MakeRotator _roll _pitch (+ (.Yaw (Math|Rotator|BreakRotator (Transformation|GetWorldRotation (Variables|/Game/DiceRuler/MapGeneration/Blueprints/BP_PuzzleMapFragment.BP_PuzzleMapFragment_C|GetStartPuzzleTrigger2 (Variables|Default|GetParentPuzzleFragment))))) 9e+01))))

(fn CreateGrid
  (bind _parentpuzzlefragment (Variables|Default|GetParentPuzzleFragment))
  (bind _fragmentsize (Variables|Default|GetFragmentSize))
  (bind (_x _y) (Math|Vector|BreakVector _fragmentsize))
  (bind _output_get (Variables|Default|SetNumberOfPuzzles (* (Variables|Default|GetGridSizeX) (Variables|Default|GetGridSizeY))))
  (if (<= _output_get 24)
    (if (== (Math|Integer|%(Integer) _output_get 2) 0)
      (Variables|Default|SetInitialPositionOnGrid (- (Transformation|GetActorLocation) (+ (* (Transformation|GetActorRightVector _parentpuzzlefragment) (/ (* _y (- (Variables|Default|GetGridSizeY) 1)) 2.0)) (* (Transformation|GetActorForwardVector _parentpuzzlefragment) (/ (* _x (- (Variables|Default|GetGridSizeX) 1)) 2.0)))))
      (for _index (range 0 (- (Variables|Default|GetGridSizeX) 1))
        (LocalVariables|SetPosOnGrid (+ (Variables|Default|GetInitialPositionOnGrid) (* (Transformation|GetActorForwardVector _parentpuzzlefragment) (* _index (LocalVariables|GetFragmentSizeX)))))
        (for _index_2 (range 0 (- (Variables|Default|GetGridSizeY) 1))
          (bind _returnvalue (Game|SpawnActorfromClass "/Game/DiceRuler/Puzzles/Memory/BP_MemoryPiece.BP_MemoryPiece_C" (Math|Conversions|ToTransform(Vector) (+ (LocalVariables|GetPosOnGrid) (* (Transformation|GetActorRightVector _parentpuzzlefragment) (* _index_2 (LocalVariables|GetFragmentSizeY))))) "Undefined" "MultiplyWithRoot" 0 0 "None" 0))
          (Utilities|Array|Add (Variables|Default|GetSpawnedFragments) _returnvalue)
          (Transformation|AttachActorToActor _returnvalue self "None" "KeepWorld" "KeepWorld" "KeepWorld" true)))
      (else
        (Development|PrintString "can't create memory puzzle, (size x* size y) should be divisible by 2")
        (return)))
    (else
      (Development|PrintString "max grid size is 24 ( because we have 12 pictures )"))))