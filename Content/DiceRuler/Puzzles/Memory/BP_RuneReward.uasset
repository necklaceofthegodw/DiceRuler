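; Rune reward actor for the Memory puzzle that shows a randomly chosen fragment image on its mesh.
; On BeginPlay it prints the game instance's current fragment images, picks one at random and applies it through a dynamic material instance with a rune color parameter.
; It then adds the image to the game instance's reward data to save and fires RewardSpawned with it.
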(event EventBeginPlay
  (bind _asbp_dice_ruler_game_instance (CallFunction|GetDiceRulerGameInstance))
  (bind _currentfragmentimages (Variables|/Game/DiceRuler/BP_DiceRulerGameInstance.BP_DiceRulerGameInstance_C|GetCurrentFragmentImages _asbp_dice_ruler_game_instance))
  (|CallParentFunction)
  (for _array_element _currentfragmentimages
    (Development|PrintString (Utilities|GetDisplayName _array_element)))
  (bind _output_get (Variables|Default|SetFragmentImage (Utilities|Array|Get(acopy) _currentfragmentimages (Math|Random|RandomIntegerinRange 0 (- (Utilities|Array|Length _currentfragmentimages) 1)))))
  (CallFunction|SetPuzzleImage _output_get 0.0)
  (Default|AddRewardDatatoSave (CallFunction|GetDiceRulerGameInstance) _output_get)
  (Default|CallRewardSpawned (Variables|Default|GetFragmentImage)))

(event Collision|EventActorBeginOverlap
  (params (OtherActor :type Actor%20Object%20Reference))
  (|CallParentFunction OtherActor) ; This node is disabled and will not be called.\nDrag off pins to build functionality.
)

(event EventTick
  (params (DeltaSeconds :type Float%20%28single-precision%29))
  (|CallParentFunction DeltaSeconds) ; This node is disabled and will not be called.\nDrag off pins to build functionality.
)

(fn ConstructionScript
  (|CallParentFunction))

(fn SetPuzzleImage
  (params (ImageToSet :type Texture%20Object%20Reference) (ColorVal :type Float%20%28single-precision%29))
  (bind _sm_mesh (Variables|Default|GetSM_Mesh))
  (bind _returnvalue (Rendering|Material|CreateDynamicMaterialInstance _sm_mesh 0 (Rendering|Material|GetMaterial _sm_mesh 0) "None" :!class /Script/Engine.PrimitiveComponent))
  (Rendering|Material|SetTextureParameterValue _returnvalue "ImageParam" ImageToSet)
  (Rendering|Material|SetScalarParameterValue _returnvalue "RuneColor" ColorVal :!class /Script/Engine.MaterialInstanceDynamic))