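; BP_PuzzleFragment is a tile actor for the Memory puzzle that shows or hides an image on a plane mesh.
; SetPuzzleImage stores the texture's name and assigns the texture to the plane through a dynamic material instance.
; SetSelected calls RevealPuzzleImage, which toggles the plane's in-game visibility, so a selected fragment shows its image.
; The box overlap events are empty.
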(event OnComponentBeginOverlap(Box)
  (params (OverlappedComponent :type Primitive%20Component%20Object%20Reference) (OtherActor :type Actor%20Object%20Reference) (OtherComp :type Primitive%20Component%20Object%20Reference) (OtherBodyIndex :type Integer) (bFromSweep :type Boolean) (SweepResult :type Hit%20Result%20Structure%20%28by%20ref%29)))

(event OnComponentEndOverlap(Box)
  (params (OverlappedComponent :type Primitive%20Component%20Object%20Reference) (OtherActor :type Actor%20Object%20Reference) (OtherComp :type Primitive%20Component%20Object%20Reference) (OtherBodyIndex :type Integer)))

(event EventBeginPlay)

(event Collision|EventActorBeginOverlap
  (params (OtherActor :type Actor%20Object%20Reference)))

(event EventTick
  (params (DeltaSeconds :type Float%20%28single-precision%29)))

(fn ConstructionScript)

(fn SetPuzzleImage
  (params (Value :type Texture%20Object%20Reference))
  (bind _plane (Variables|Default|GetPlane))
  (Variables|Default|SetImageNameString (Utilities|GetObjectName Value))
  (bind _returnvalue (Rendering|Material|CreateDynamicMaterialInstance _plane 0 (Rendering|Material|GetMaterial _plane 0) "None" :!class /Script/Engine.PrimitiveComponent))
  (Rendering|Material|SetTextureParameterValue _returnvalue "ImageParam" Value))

(fn RevealPuzzleImage
  (params (IsRevealed :type Boolean))
  (Development|SetHiddeninGame (Variables|Default|GetPlane) (not IsRevealed) false))

(fn SetSelected
  (params (IsSelected :type Boolean))
  (CallFunction|RevealPuzzleImage IsSelected))