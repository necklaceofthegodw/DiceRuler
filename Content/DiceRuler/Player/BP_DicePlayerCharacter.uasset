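; Player character for DiceRuler that carries puzzle items and exposes camera controls.
; Pickup frees the overlapped item from any balance scale, disables its physics and uses a timeline to lerp it to WeaponSocket before attaching; dropping restores physics.
; Camera functions pan along the map fragment manager's axes, set spring arm length and reset to a saved location and default zoom.
; Attack is empty, and the sword spawn and attack logic is disconnected.
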(event Custom|Attack)

(event Custom|TryPickingUpItem
  (bind _itemoverlapping (Variables|Default|GetItemOverlapping))
  (bind _balancescale (Variables|/Game/DiceRuler/Gameplay/Pickables/BP_PickableItem.BP_PickableItem_C|GetBalanceScale _itemoverlapping))
  (if (not (Variables|Default|GetIsPickingUp))
    (if (not (== (Variables|Default|GetItemOverlapping) (Variables|Default|GetPickedItem)))
      (Utilities|IsValid (Variables|Default|GetPickedItem)
        (:Is%20Not%20Valid
          (Utilities|IsValid _itemoverlapping
            (:Is%20Valid
              ;[1 1 1] TODO add event on item picked, that the balance scale will listen to and update sockets occupied by pickables
              (Utilities|IsValid _balancescale
                (:Is%20Valid
                  (Default|RemoveItemfromSocket _balancescale _itemoverlapping))
                (:Is%20Not%20Valid
                  _))
              (Variables|Default|SetPickedItem (Variables|Default|GetItemOverlapping))
              (Variables|Default|SetIsPickingUp true)
              (Default|ShowInteractionWidget (Variables|Default|GetPickedItem) false)
              (Physics|SetSimulatePhysics (Variables|/Game/DiceRuler/Gameplay/Pickables/BP_PickableItem.BP_PickableItem_C|GetSM_Mesh (Variables|Default|GetPickedItem)) false)
              (Collision|SetCollisionEnabled (Variables|/Game/DiceRuler/Gameplay/Pickables/BP_PickableItem.BP_PickableItem_C|GetSM_Mesh (Variables|Default|GetPickedItem)) "NoCollision")
              (bind _position (Timeline|Timeline_Pickup PlayFromStart)
                (:Update
                  (Transformation|SetActorLocation (Variables|Default|GetPickedItem) (Math|Vector|Lerp(Vector) (Transformation|GetActorLocation (Variables|Default|GetPickedItem)) (Transformation|GetSocketLocation (Variables|Character|GetMesh) "WeaponSocket") _position) false false))
                (:Finished
                  (Transformation|AttachComponentToComponent (Variables|Default|GetPickedItem) (Variables|Character|GetMesh) "WeaponSocket" "SnapToTarget" "SnapToTarget" "KeepRelative" true)
                  (Variables|Default|SetIsPickingUp false))))))))))

(event Custom|TryDroppingItem
  (if (not (Variables|Default|GetIsPickingUp))
    (Utilities|IsValid (Variables|Default|GetPickedItem)
      (:Is%20Valid
        (Transformation|DetachFromActor (Variables|Default|GetPickedItem) "KeepWorld" "KeepWorld" "KeepWorld")
        (Collision|SetCollisionEnabled (Variables|/Game/DiceRuler/Gameplay/Pickables/BP_PickableItem.BP_PickableItem_C|GetSM_Mesh (Variables|Default|GetPickedItem)) "QueryAndPhysics")
        (Physics|SetSimulatePhysics (Variables|/Game/DiceRuler/Gameplay/Pickables/BP_PickableItem.BP_PickableItem_C|GetSM_Mesh (Variables|Default|GetPickedItem)) true)
        (Variables|Default|SetPickedItem 0)))))

(event EventBeginPlay
  (|CallParentFunction))

(fn ConstructionScript)

(fn ChangeCameraArmLength
  (params (lengthToSet :type Float%20%28double-precision%29))
  (Variables|/Script/Engine.SpringArmComponent|SetTargetArmLength (Variables|Camera|GetSpringArm) lengthToSet))

(fn AttachSword
  (bind _returnvalue (Game|SpawnActorfromClass "/Game/DiceRuler/Puzzles/Sokoban/Sword/BP_Sword.BP_Sword_C" (Transformation|GetActorTransform) "Undefined" "MultiplyWithRoot" 0 0))
  (Transformation|AttachComponentToComponent _returnvalue (Variables|Character|GetMesh) "WeaponSocket" "SnapToTarget" "SnapToTarget" "KeepRelative" true)
  (Variables|Default|SetAttachedSword _returnvalue)
  (Collision|SetCollisionEnabled (Variables|/Game/DiceRuler/Puzzles/Sokoban/Sword/BP_Sword.BP_Sword_C|GetCapsule (Variables|Default|GetAttachedSword)) "NoCollision"))

(fn SetActivePuzzle
  (params (CurrentMapFragment :type BP%20Map%20Fragment%20Object%20Reference))
  (Variables|Default|SetCurrent%20Map%20Fragment CurrentMapFragment))

(fn MoveCameraXAxis
  (params (val :type Float%20%28double-precision%29))
  (Transformation|AddWorldOffset (Variables|Camera|GetCamera) (* (Transformation|GetActorForwardVector (CallFunction|GetDiceMapFragmentManager)) (* val (Variables|Default|GetCameraMoveSpeed))) false false))

(fn MoveCameraYAxis
  (params (val :type Float%20%28double-precision%29))
  (Transformation|AddWorldOffset (Variables|Camera|GetCamera) (* (Transformation|GetActorRightVector (CallFunction|GetDiceMapFragmentManager)) (* val (Variables|Default|GetCameraMoveSpeed))) false false))

(fn ResetCameraPosition
  (Transformation|SetWorldLocation (Variables|Camera|GetCamera) (Variables|Default|GetInitialCameraLocation) false false)
  (Variables|/Game/DiceRuler/Player/BP_DicePlayerController.BP_DicePlayerController_C|SetScrollVal (CallFunction|GetDicePlayerController) 0.5)
  (Input|ChangeCameraArmLength (CallFunction|GetDicePlayerCharacter) 3.35e+03))

(fn SetInitialCameraLocation
  (Variables|Default|SetInitialCameraLocation (Transformation|GetWorldLocation (Variables|Camera|GetCamera))))