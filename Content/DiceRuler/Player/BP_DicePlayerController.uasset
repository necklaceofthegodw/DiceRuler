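; Player controller for the dice character that routes Enhanced Input actions according to the current input mode: Gameplay, Puzzle or Map Generation.
; Gameplay adds hold-to-follow and short-click move-to-cursor plus right-click attack, while sharing item pickup, drop and trajectory-timed throwing with Puzzle.
; Map Generation forwards exit selection, confirm and build-exit to the map fragment manager, and Puzzle clicks fire ClickedSomething.
; Scroll zooms the camera arm in any mode.
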(event Input|EnhancedActionEvents|EnhancedInputActionIA_Click
  (params (ActionValue :type Boolean) (ElapsedSeconds :type Float%20%28double-precision%29) (TriggeredSeconds :type Float%20%28double-precision%29) (InputAction :type Input%20Action%20Object%20Reference :default "/Game/TopDown/Input/Actions/IA_Click.IA_Click"))
  (bind _inputmode (CallFunction|GetCurrentInputMode))
  ;[0.05098 0.05098 0.05098] Set Destination Input - Gamepad and Mouse - On Released, if input wasn't held, try to move the possessed character to Current Move Field object
  (:Triggered
    (switch Utilities|FlowControl|Switch|SwitchonE_InputMode _inputmode
      (:NewEnumerator0
        (bind _output_get (Variables|Input|SetCachedDestination (CallFunction|GetLocationUnderCursor)))
        (CallFunction|Follow _output_get))))
  (:Started
    (switch Utilities|FlowControl|Switch|SwitchonE_InputMode _inputmode
      (:NewEnumerator0
        (AI|Navigation|StopMovement))
      (:NewEnumerator1
        (Default|TrySelectExit (Variables|Default|GetMapFragmentManager) self))
      (:NewEnumerator3
        (Default|CallClickedSomething))))
  (:Canceled
    (switch Utilities|FlowControl|Switch|SwitchonE_InputMode _inputmode :!label _label
      (:NewEnumerator0
        (if (< ElapsedSeconds (Variables|Input|GetPressedThreshold))
          (Variables|Input|SetCachedDestination (CallFunction|GetLocationUnderCursor))
          (Default|Moveto (Variables|Default|GetBP_MovementComponent) (Variables|Input|GetCachedDestination))))))
  (:Completed
    (goto _label)))

(event Input|EnhancedActionEvents|EnhancedInputActionIA_Confirm
  (params (ActionValue :type Boolean) (ElapsedSeconds :type Float%20%28double-precision%29) (TriggeredSeconds :type Float%20%28double-precision%29) (InputAction :type Input%20Action%20Object%20Reference :default "/Game/TopDown/Input/Actions/IA_Confirm.IA_Confirm"))
  (:Started
    (switch Utilities|FlowControl|Switch|SwitchonE_InputMode (CallFunction|GetCurrentInputMode)
      (:NewEnumerator1
        (Default|ChecktoSpawnNextFragment (Variables|Default|GetMapFragmentManager))))))

(event Input|EnhancedActionEvents|EnhancedInputActionIA_Scroll
  (params (ActionValue :type Float%20%28double-precision%29) (ElapsedSeconds :type Float%20%28double-precision%29) (TriggeredSeconds :type Float%20%28double-precision%29) (InputAction :type Input%20Action%20Object%20Reference :default "/Game/TopDown/Input/Actions/IA_Scroll.IA_Scroll"))
  ;[1 1 1] Wheel scroll - zoom in/out
  (Variables|Default|SetScrollVal (Math|Float|Clamp(Float) (+ (Variables|Default|GetScrollVal) (* ActionValue -0.05))))
  (Default|ChangeCameraArmLength (CallFunction|GetDicePlayerCharacter) (Math|Float|Lerp 7e+02 6e+03 (Variables|Default|GetScrollVal))))

(event Input|EnhancedActionEvents|EnhancedInputActionIA_RightClick
  (params (ActionValue :type Boolean) (ElapsedSeconds :type Float%20%28double-precision%29) (TriggeredSeconds :type Float%20%28double-precision%29) (InputAction :type Input%20Action%20Object%20Reference :default "/Game/TopDown/Input/Actions/IA_RightClick.IA_RightClick"))
  (switch Utilities|FlowControl|Switch|SwitchonE_InputMode (CallFunction|GetCurrentInputMode)
    (:NewEnumerator0
      (Default|Attack (Variables|Default|GetDicePlayerCharacter)))))

(event Input|EnhancedActionEvents|EnhancedInputActionIA_ExitBuild
  (params (ActionValue :type Boolean) (ElapsedSeconds :type Float%20%28double-precision%29) (TriggeredSeconds :type Float%20%28double-precision%29) (InputAction :type Input%20Action%20Object%20Reference :default "/Game/TopDown/Input/Actions/IA_ExitBuild.IA_ExitBuild"))
  (:Started
    (switch Utilities|FlowControl|Switch|SwitchonE_InputMode (CallFunction|GetCurrentInputMode)
      (:NewEnumerator1
        (Default|ExitBuildMode (Variables|Default|GetMapFragmentManager))))))

(event Input|EnhancedActionEvents|EnhancedInputActionIA_Throw
  (params (ActionValue :type Boolean) (ElapsedSeconds :type Float%20%28double-precision%29) (TriggeredSeconds :type Float%20%28double-precision%29) (InputAction :type Input%20Action%20Object%20Reference :default "/Game/TopDown/Input/Actions/IA_Throw.IA_Throw"))
  (bind _dice_player_character (CallFunction|GetDicePlayerCharacter))
  (bind _shootingcomponent (Variables|/Game/DiceRuler/Player/BP_DicePlayerCharacter.BP_DicePlayerCharacter_C|GetShootingComponent _dice_player_character))
  (:Started
    (switch Utilities|FlowControl|Switch|SwitchonE_InputMode (CallFunction|GetCurrentInputMode)
      (:NewEnumerator0
        _)
      (:NewEnumerator3
        _))
    (Default|StartBallTrajectoryTimer _shootingcomponent))
  (:Completed
    (switch Utilities|FlowControl|Switch|SwitchonE_InputMode (CallFunction|GetCurrentInputMode)
      (:NewEnumerator0
        _)
      (:NewEnumerator3
        _))
    (Default|StopBallTrajectoryTimer _shootingcomponent)
    (Default|Shot _shootingcomponent)))

(event Input|EnhancedActionEvents|EnhancedInputActionIA_Interact
  (params (ActionValue :type Boolean) (ElapsedSeconds :type Float%20%28double-precision%29) (TriggeredSeconds :type Float%20%28double-precision%29) (InputAction :type Input%20Action%20Object%20Reference :default "/Game/TopDown/Input/Actions/IA_Interact.IA_Interact"))
  (:Started
    (switch Utilities|FlowControl|Switch|SwitchonE_InputMode (CallFunction|GetCurrentInputMode)
      (:NewEnumerator0
        _)
      (:NewEnumerator3
        _))
    (Default|TryPickingUpItem (CallFunction|GetDicePlayerCharacter))))

(event Input|EnhancedActionEvents|EnhancedInputActionIA_DropItem
  (params (ActionValue :type Boolean) (ElapsedSeconds :type Float%20%28double-precision%29) (TriggeredSeconds :type Float%20%28double-precision%29) (InputAction :type Input%20Action%20Object%20Reference :default "/Game/TopDown/Input/Actions/IA_DropItem.IA_DropItem"))
  (:Started
    (switch Utilities|FlowControl|Switch|SwitchonE_InputMode (CallFunction|GetCurrentInputMode)
      (:NewEnumerator0
        _)
      (:NewEnumerator3
        _))
    (Default|TryDroppingItem (CallFunction|GetDicePlayerCharacter))))

(event EventBeginPlay
  (bind _returnvalue (PlayerController|LocalPlayerSubsystems|GetEnhancedInputLocalPlayerSubsystem))
  ;[0.05098 0.05098 0.05098] Add Mapping Context
  (Utilities|IsValid _returnvalue
    (:Is%20Valid
      (Input|AddMappingContext _returnvalue "/Game/TopDown/Input/IMC_Default.IMC_Default" 0 "(bIgnoreAllPressedKeysUntilRelease=True,bForceImmediately=False,bNotifyUserSettings=False)")
      (bind _returnvalue_2 (Actor|GetActorOfClass "/Game/DiceRuler/MapGeneration/Blueprints/BP_MapFragmentManager.BP_MapFragmentManager_C"))
      (Variables|Default|SetMapFragmentManager _returnvalue_2)
      (bind _asbp_dice_player_character (Utilities|Casting|CastToBP_DicePlayerCharacter (Pawn|GetControlledPawn)))
      (Variables|Default|SetDicePlayerCharacter _asbp_dice_player_character))))

(fn ConstructionScript)

(fn Moveto
  (params (Location :type Vector))
  (AI|Navigation|SimpleMovetoLocation self Location)
  (Niagara|SpawnSystematLocation (Variables|Input|GetFXCursor) Location))

(fn Follow
  (params (Location :type Vector))
  (bind _returnvalue (Pawn|GetControlledPawn))
  (Pawn|Input|AddMovementInput _returnvalue (Math|Vector|GetUnitDirection(Vector) (Transformation|GetActorLocation _returnvalue) Location) 1.0 false))

(fn GetLocationUnderCursor
  (bind _hitresult (Game|Player|GetHitResultUnderCursorbyChannel "TraceTypeQuery1" true))
  (bind (_bblockinghit _binitialoverlap _time _distance _location) (Collision|BreakHitResult _hitresult))
  (if _bblockinghit
    (return _location)
    (else
      (return "0, 0, 0"))))

(fn GetLocationUnderFinger
  (bind _hitresult (Class|PlayerController|GetHitResultUnderFingerbyChannel "Touch1" "TraceTypeQuery1" false))
  (bind (_bblockinghit _binitialoverlap _time _distance _location) (Collision|BreakHitResult _hitresult))
  (return _bblockinghit _location))

(fn CheckActorUnderCursor
  (bind _returnvalue (Game|GetPlayerController 0))
  (bind (_hitresult _returnvalue_2) (Game|Player|GetHitResultUnderCursorbyChannel _returnvalue "TraceTypeQuery1" true))
  (if _returnvalue_2
    (return (.HitActor (Collision|BreakHitResult _hitresult)))
    (else
      (return 0))))