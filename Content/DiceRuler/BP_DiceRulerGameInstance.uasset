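; Game instance for DiceRuler that owns the map fragment save game and tracks the input mode and saved flag.
; On Init it loads the save slot or creates a new save object.
; Add and remove events edit the stored fragment structs and write the slot immediately, while SaveCurrentMapFragments only copies the manager's spawned fragments into the save object.
; RecreateMapFragments respawns BP_MapFragment actors from saved data; DeleteSave clears the slot.
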(event Custom|AddMapFragmentDataToSave
  (params (S_MapFragment :type S%20Map%20Fragment%20Structure%20%28by%20ref%29))
  (bind _bp_savegame (Variables|Default|GetBP_SaveGame))
  (Utilities|Array|Add (Variables|/Game/DiceRuler/Savegame/BP_SaveGame.BP_SaveGame_C|GetMapFragments _bp_savegame) S_MapFragment)
  (SaveGame|SaveGametoSlot _bp_savegame (Variables|Default|GetSavedGameSlotName)))

(event Custom|RemoveMapFragmentDataFromSave
  (params (S_MapFragment :type S%20Map%20Fragment%20Structure%20%28by%20ref%29))
  (bind _bp_savegame (Variables|Default|GetBP_SaveGame))
  (Utilities|Array|RemoveItem (Variables|/Game/DiceRuler/Savegame/BP_SaveGame.BP_SaveGame_C|GetMapFragments _bp_savegame) S_MapFragment)
  (SaveGame|SaveGametoSlot _bp_savegame (Variables|Default|GetSavedGameSlotName)))

(event EventInit
  (Variables|Default|SetInputMode "NewEnumerator0")
  (Saving|LoadMapFragments))

(fn ChangeInputMode
  (params (InputMode :type E_InputMode%20Enum :default "NewEnumerator0"))
  (Variables|Default|SetInputMode InputMode))

(fn LoadMapFragments
  (bind _savedgameslotname (Variables|Default|GetSavedGameSlotName))
  (bind _returnvalue (SaveGame|DoesSaveGameExist _savedgameslotname))
  (if _returnvalue
    (bind _returnvalue_2 (SaveGame|LoadGamefromSlot _savedgameslotname))
    (bind _asbp_save_game (Utilities|Casting|CastToBP_SaveGame _returnvalue_2))
    (Variables|Default|SetBP_SaveGame _asbp_save_game)
    (else
      (bind _returnvalue_3 (SaveGame|CreateSaveGameObject "/Game/DiceRuler/Savegame/BP_SaveGame.BP_SaveGame_C"))
      (Variables|Default|SetBP_SaveGame _returnvalue_3)
      (Development|PrintString "create save slot"))))

(fn RecreateMapFragments
  (for _array_element (Variables|/Game/DiceRuler/Savegame/BP_SaveGame.BP_SaveGame_C|GetMapFragments (Variables|BP_DiceRulerGameInstance_C|GetBP_SaveGame (CallFunction|GetDiceRulerGameInstance)))
    (bind _returnvalue (Game|SpawnActorfromClass "/Game/DiceRuler/MapGeneration/Blueprints/BP_MapFragment.BP_MapFragment_C" (.transform _array_element) "Undefined" "MultiplyWithRoot" 0 (Utilities|Struct|MakeS_MapFragment (.isstartingfragment _array_element) (.exits _array_element) (.exitsthatareconnected _array_element) (.transform _array_element)) false 0))
    (Utilities|Array|Add (LocalVariables|GetFragments) _returnvalue))
  (Development|PrintString "respawn map fragments from save")
  (return (LocalVariables|GetFragments)))

(fn SaveCurrentMapFragments
  (for _array_element (Variables|/Game/DiceRuler/MapGeneration/Blueprints/BP_MapFragmentManager.BP_MapFragmentManager_C|GetSpawnedMapFragments (CallFunction|GetDiceMapFragmentManager))
    (Utilities|Array|Add (LocalVariables|GetMapFragments) (Utilities|Struct|MakeS_MapFragment (.IsStartingFragment (Utilities|Struct|BreakS_MapFragment (Variables|/Game/DiceRuler/MapGeneration/Blueprints/BP_MapFragment.BP_MapFragment_C|GetMapFragmentInfo _array_element))) (.Exits (Utilities|Struct|BreakS_MapFragment (Variables|/Game/DiceRuler/MapGeneration/Blueprints/BP_MapFragment.BP_MapFragment_C|GetMapFragmentInfo _array_element))) (.ExitsThatAreConnected (Utilities|Struct|BreakS_MapFragment (Variables|/Game/DiceRuler/MapGeneration/Blueprints/BP_MapFragment.BP_MapFragment_C|GetMapFragmentInfo _array_element))) (Transformation|GetActorTransform _array_element))))
  (Variables|/Game/DiceRuler/Savegame/BP_SaveGame.BP_SaveGame_C|SetMapFragments (Variables|Default|GetBP_SaveGame) (LocalVariables|GetMapFragments)))

(fn DeleteSave
  (SaveGame|DeleteGameinSlot (Variables|Default|GetSavedGameSlotName)))

(fn SetIsGameSaved
  (params (bIsGameSaved :type Boolean))
  (Variables|Default|SetbIsGameSaved bIsGameSaved))