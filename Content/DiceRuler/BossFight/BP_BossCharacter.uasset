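; Boss character for the DiceRuler boss fight that periodically fires a radial burst of snow bullets.
; Tick accumulates time and calls SphereAttack every TimeBetweenSpawns, which rotates a Sphere component in even yaw steps to spawn TracesNum bullets in a ring.
; Each bullet receives a physics force pointing from its spawn point back through the boss's center.
; A separate Attack event plays the magic montage, guarded by IsAttacking, without triggering the burst.
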(event EventBeginPlay)

(event Collision|EventActorBeginOverlap
  (params (OtherActor :type Actor%20Object%20Reference)))

(event EventTick
  (params (DeltaSeconds :type Float%20%28single-precision%29))
  (Variables|Default|SetTimeElapsed (+ (Variables|Default|GetTimeElapsed) DeltaSeconds))
  (if (> (Variables|Default|GetTimeElapsed) (Variables|Default|GetTimeBetweenSpawns))
    (CallFunction|SphereAttack)
    (Variables|Default|SetTimeElapsed 0.0)))

(event EventAttack
  (if (not (Variables|Default|GetIsAttacking))
    (Animation|Montage|PlayMontage (Variables|Character|GetMesh) "/Game/DiceRuler/BossFight/Vampire/Animations/MagicAttackMontage.MagicAttackMontage"
      (:then
        (Variables|Default|SetIsAttacking true))
      (:OnCompleted
        (Variables|Default|SetIsAttacking false)))))

(fn ConstructionScript)

(fn SphereAttack
  (bind _returnvalue (Transformation|GetActorLocation))
  (bind _sphere (Variables|Default|GetSphere))
  (bind _returnvalue_2 (Math|Vector|GetForwardVector _sphere))
  (bind _returnvalue_3 (* _returnvalue_2 5e+01))
  (bind _returnvalue_4 (+ _returnvalue _returnvalue_3))
  (for _index (range 0 (- (LocalVariables|GetTracesNum) 1))
    (Transformation|SetRelativeRotation (Variables|Default|GetSphere) (Math|Rotator|MakeRotator 0.0 0.0 (Math|Conversions|ToFloat(Integer) (* _index (/ (Math|Float|MakeLiteralFloat 3.6e+02) (LocalVariables|GetTracesNum))))) false false)
    (bind _returnvalue_5 (Game|SpawnActorfromClass "/Game/DiceRuler/BossFight/Barrel/BP_SnowBullet.BP_SnowBullet_C" (Math|Conversions|ToTransform(Vector) _returnvalue_4) "Undefined" "MultiplyWithRoot" 0 0))
    (Physics|AddForce (Variables|/Game/DiceRuler/BossFight/Barrel/BP_SnowBullet.BP_SnowBullet_C|GetStaticMesh _returnvalue_5) (* (- _returnvalue _returnvalue_4) 1e+03) "None" false)))