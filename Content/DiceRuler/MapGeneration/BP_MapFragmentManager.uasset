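; Map manager that spawns the starting fragment and runs a build mode for expanding the map from the player's fragment.
; It spawns a ghost fragment near the player with a random exit layout, flagging encounters on exits after the first.
; Selected exit pairs snap together through per-socket rotation lookup tables and a location offset.
; Spawning repeats until three fragments are counted or no free exits remain, then build mode closes.
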(event EventBeginPlay
  (CallFunction|SpawnFirstMapFragment))

(event Collision|EventActorBeginOverlap
  (params (OtherActor :type Actor%20Object%20Reference)))

(event EventTick
  (params (DeltaSeconds :type Float%20%28single-precision%29)))

(fn ConstructionScript)

(fn SpawnMapFragments
  (bind _output_get (LocalVariables|SetCurrentExitConfig (Utilities|Select :Index (Math|Random|RandomIntegerinRange 0 4) :Option%200 (LocalVariables|GetExitsConfig) :Option%201 (LocalVariables|GetExitsConfig_0) :Option%202 (LocalVariables|GetExitsConfig_1) :Option%203 (LocalVariables|GetExitsConfig_2) :Option%204 (LocalVariables|GetExitsConfig_3))))
  ;[1 1 1] Add encounter to the second existing exit
  (for (_array_element _array_index) _output_get
    (if _array_element
      (if (LocalVariables|GetFirstExistingExit)
        (Utilities|Array|SetArrayElem (LocalVariables|GetEncounters) _array_index true)
        (else
          (LocalVariables|SetFirstExistingExit true)))))
  (bind _asbp_top_down_character (Utilities|Casting|CastToBP_TopDownCharacter (Game|Player|GetPlayerPawn 0)))
  (bind _returnvalue (Game|SpawnActorfromClass "/Game/DiceRuler/MapGeneration/BP_MapFragment.BP_MapFragment_C" (Math|Transform|MakeTransform (+ (.Location (Math|Transform|BreakTransform (Transformation|GetActorTransform _asbp_top_down_character))) "-300.000000,240.000000,-50.000000")) "Undefined" "MultiplyWithRoot" 0 (Utilities|Struct|MakeS_MapFragment false (LocalVariables|GetCurrentExitConfig) (LocalVariables|GetEncounters)) true 0))
  (bind _output_get_2 (Variables|Default|SetCurrentlySpawnedFragment _returnvalue))
  (bind _outmapfragment (CallFunction|GetDicePlayerMapFragment))
  (Variables|Default|SetPlayerMapFragment _outmapfragment)
  (Utilities|Array|Add (Variables|Default|GetSpawnedMapFragments) _output_get_2))

(fn SpawnFirstMapFragment
  (bind _returnvalue (Game|SpawnActorfromClass "/Game/DiceRuler/MapGeneration/BP_MapFragment.BP_MapFragment_C" (Transformation|GetActorTransform) "Undefined" "MultiplyWithRoot" 0 (Variables|Default|GetMap%20Fragment%20Info) false 0))
  (bind _output_get (Variables|Default|SetFirstMapFragment _returnvalue))
  (Default|InitEncounters _output_get)
  (Utilities|Array|Add (Variables|Default|GetSpawnedMapFragments) _output_get))

(fn TrySelectExit
  (params (PlayerController :type Player%20Controller%20Object%20Reference))
  (bind _playermapfragment (Variables|Default|GetPlayerMapFragment))
  (bind _playermapfragment_2 (Variables|Default|GetPlayerMapFragment))
  (bind _currentlyspawnedfragment (Variables|Default|GetCurrentlySpawnedFragment))
  (bind _asbp_exit (Utilities|Casting|CastToBP_Exit (.HitActor (Collision|BreakHitResult (.HitResult (Game|Player|GetHitResultUnderCursorbyChannel PlayerController "TraceTypeQuery1" true))))))
  (Utilities|IsValid (Variables|Default|GetFirstSelectedExit)
    (:Is%20Valid
      (Utilities|IsValid (Variables|Default|GetSecondSelectedExit)
        (:Is%20Not%20Valid
          (Utilities|IsValid _playermapfragment
            (:Is%20Valid
              (bind _outselectedexit (Default|SelectExit _playermapfragment _asbp_exit))
              (Variables|Default|SetSecondSelectedExit _outselectedexit))))))
    (:Is%20Not%20Valid
      (Utilities|IsValid _currentlyspawnedfragment
        (:Is%20Valid
          (bind _outselectedexit_2 (Default|SelectExit _currentlyspawnedfragment _asbp_exit))
          (Variables|Default|SetFirstSelectedExit _outselectedexit_2)
          (Utilities|IsValid _playermapfragment_2
            (:Is%20Valid
              (Default|ShowBuildingDecal _playermapfragment_2 true))))))))

(fn ConnectMapFragments
  (bind _secondselectedexit (Variables|Default|GetSecondSelectedExit))
  (bind _firstselectedexit (Variables|Default|GetFirstSelectedExit))
  (bind _firstselectedexit_2 (Variables|Default|GetFirstSelectedExit))
  (bind _parentmapfragment (Variables|/Game/DiceRuler/MapGeneration/BP_SelectableObject.BP_SelectableObject_C|GetParentMapFragment _firstselectedexit))
  (if (and (Utilities|IsValid (Variables|Default|GetFirstSelectedExit)) (Utilities|IsValid (Variables|Default|GetSecondSelectedExit)))
    (LocalVariables|SetSelectedExit_AndRotations (Utilities|Select :Index (Utilities|Array|FindItem (Transformation|GetAllSocketNames (Variables|/Game/DiceRuler/MapGeneration/BP_MapFragment.BP_MapFragment_C|GetSM_Brick (Variables|/Game/DiceRuler/MapGeneration/BP_SelectableObject.BP_SelectableObject_C|GetParentMapFragment _firstselectedexit_2))) (Variables|/Game/DiceRuler/MapGeneration/BP_SelectableObject.BP_SelectableObject_C|GetAttachSocketName _firstselectedexit_2)) :Option%200 (LocalVariables|GetSocketExit_0_AndRotations) :Option%201 (LocalVariables|GetSocketExit_1_AndRotations) :Option%202 (LocalVariables|GetSocketExit_2_AndRotations) :Option%203 (LocalVariables|GetSocketExit_3_AndRotations) :Option%204 (LocalVariables|GetSocketExit_4_AndRotations) :Option%205 (LocalVariables|GetSocketExit_5_AndRotations)))
    (Transformation|SetActorRotation _parentmapfragment (.Value (Utilities|Map|Find (LocalVariables|GetSelectedExit_AndRotations) (Variables|/Game/DiceRuler/MapGeneration/BP_SelectableObject.BP_SelectableObject_C|GetAttachSocketName _secondselectedexit))))
    (Transformation|SetActorLocation _parentmapfragment (+ (Transformation|GetActorLocation _secondselectedexit) (- (Transformation|GetActorLocation _parentmapfragment) (Transformation|GetActorLocation _firstselectedexit))) false false)
    (Default|SetHighlight (Variables|Default|GetFirstSelectedExit) "NewEnumerator0")
    (Default|SetCollsionEnableinExits (Variables|/Game/DiceRuler/MapGeneration/BP_SelectableObject.BP_SelectableObject_C|GetParentMapFragment (Variables|Default|GetFirstSelectedExit)) false)
    (Collision|SetActorEnableCollision (Variables|Default|GetSecondSelectedExit) false)
    (else
      (Development|PrintString "try connecting exits not selected"))))

(fn GetPlayerMapFragment
  (bind _bp_topdowncharacter (CallFunction|GetDicePlayerCharacter))
  (bind _returnvalue (Transformation|GetActorLocation _bp_topdowncharacter))
  (bind _outhit (Collision|LineTraceForObjects _returnvalue (+ _returnvalue "0.000000,0.000000,-200.000000") (Utilities|Array|MakeArray "ObjectTypeQuery2" "ObjectTypeQuery1") false 0 "Persistent"))
  (bind _asbp_map_fragment (Utilities|Casting|CastToBP_MapFragment (.HitActor (Collision|BreakHitResult _outhit))))
  (Variables|Default|SetPlayerMapFragment _asbp_map_fragment))

(fn ExitBuildMode
  (Default|ChangeInputMode (CallFunction|GetDiceRulerGameInstance) "NewEnumerator0")
  (Default|ShowExploreMenuWidget (Variables|/Game/DiceRuler/HUD/BP_DiceRulerHUD.BP_DiceRulerHUD_C|GetWBP_HUD (CallFunction|GetDiceHud)) false)
  (Default|CallBuildModeClosed))

(fn ChecktoSpawnNextFragment
  (bind _playermapfragment (Variables|Default|GetPlayerMapFragment))
  (bind _spawnedfragmentscount (Variables|Default|GetSpawnedFragmentsCount))
  (Math|Integer|IncrementInt _spawnedfragmentscount
    (:%20%20
      (CallFunction|ConnectMapFragments)
      (if (== _spawnedfragmentscount 3)
        (CallFunction|ExitBuildMode :!label _label)
        (else
          (bind _outunconnectedexits (Default|FindUnConnectedExits (Variables|Default|GetPlayerMapFragment)))
          (if (> (Utilities|Array|Length _outunconnectedexits) 0)
            (Variables|Default|SetFirstSelectedExit 0)
            (Variables|Default|SetSecondSelectedExit 0)
            (Variables|/Game/DiceRuler/MapGeneration/BP_MapFragment.BP_MapFragment_C|SetHighlightedExit _playermapfragment 0)
            (Variables|/Game/DiceRuler/MapGeneration/BP_MapFragment.BP_MapFragment_C|SetSelectedExit _playermapfragment 0)
            (CallFunction|SpawnMapFragments)
            (else
              (goto _label))))))))

(fn EnableExitsinAllMapFragments
  (params (bNewActorEnableCollision :type Boolean))
  (for _array_element (Variables|Default|GetSpawnedMapFragments)
    (Default|SetCollsionEnableinExits _array_element bNewActorEnableCollision)))