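; Movement component for the top-down controller that finds and highlights the move fields the player can reach from the current dice map fragment.
; FindMoveFieldsInRange enables all fragment exits, then line-traces from below the pawn along the fragment's four horizontal axes.
; Each exit hit starts a second trace onward in that direction, and any move field hit is stored and highlighted.
; Debug traces and prints show the results.
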(event EventBeginPlay
  (bind _asbp_top_down_controller (Utilities|Casting|CastToBP_TopDownController (Components|GetOwner)))
  (Variables|Default|SetBP_TopDownController _asbp_top_down_controller))

(event EventTick
  (params (DeltaSeconds :type Float%20%28single-precision%29)))

(fn FindMoveFieldsinRange
  (Utilities|FlowControl|Sequence
    (:then_0
      (Default|EnableExitsinAllMapFragments (CallFunction|GetDiceMapFragmentManager) true))
    (:then_1
      (bind _outmapfragment (CallFunction|GetDicePlayerMapFragment))
      (Variables|Default|SetPlayer%20Map%20Fragment _outmapfragment)
      (Utilities|Array|Clear (Variables|Default|GetBP_MoveFieldsAvailable)))
    (:then_2
      (LocalVariables|SetTraceDirectionVectors (Utilities|Array|MakeArray (Transformation|GetActorRightVector (Variables|Default|GetPlayer%20Map%20Fragment)) (Math|Vector|NegateVector (Transformation|GetActorRightVector (Variables|Default|GetPlayer%20Map%20Fragment))) (Transformation|GetActorForwardVector (Variables|Default|GetPlayer%20Map%20Fragment)) (Math|Vector|NegateVector (Transformation|GetActorForwardVector (Variables|Default|GetPlayer%20Map%20Fragment)))))
      (LocalVariables|SetStartLocation (+ (Transformation|GetActorLocation (Pawn|GetControlledPawn (Variables|Default|GetBP_TopDownController))) "0.000000,0.000000,-80.000000")))
    (:then_3
      (for _array_element (LocalVariables|GetTraceDirectionVectors)
        (bind _outhit (Collision|LineTraceByChannel (LocalVariables|GetStartLocation) (+ (LocalVariables|GetStartLocation) (* _array_element (LocalVariables|GetTraceDistance))) "TraceTypeQuery1" false 0 "ForDuration"))
        (bind _asbp_exit (Utilities|Casting|CastToBP_Exit (.HitActor (Collision|BreakHitResult _outhit)))
          (:then
            (bind _output_get (LocalVariables|SetExitToIgnore _asbp_exit))
            (Development|PrintString (Utilities|String|Append "  exit to ignore :  " (Utilities|GetDisplayName _output_get)))
            (bind _outhit_2 (Collision|LineTraceByChannel (+ (Transformation|GetActorLocation (LocalVariables|GetExitToIgnore)) 2e+01) (+ (Transformation|GetActorLocation (LocalVariables|GetExitToIgnore)) (* _array_element 2e+02)) "TraceTypeQuery1" false 0 "ForDuration" true "(R=0.685470,G=0.021701,B=0.833333,A=1.000000)"))
            (bind _asbp_move_field (Utilities|Casting|CastToBP_MoveField (.HitActor (Collision|BreakHitResult _outhit_2))))
            (Utilities|Array|Add (Variables|Default|GetBP_MoveFieldsAvailable) _asbp_move_field)
            (Development|PrintString (Utilities|String|Append "move field hit: " (Utilities|GetDisplayName _asbp_move_field))))
          (:CastFailed
            (Development|PrintString "no exit -> cant move in this direction")))))
    (:then_4
      (for _array_element_2 (Variables|Default|GetBP_MoveFieldsAvailable)
        (Default|SetHighlight _array_element_2 "NewEnumerator1")))))