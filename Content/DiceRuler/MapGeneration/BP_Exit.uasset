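; BP_Exit is an exit actor for DiceRuler's map generation that tracks whether it is connected to another exit.
; Overlapping another BP_Exit prints a debug message and sets the IsConnected flag, which a same-named function returns.
; An author TODO doubts that this detection works, because exits have collision disabled after connecting.
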(event EventBeginPlay
  (|CallParentFunction) ; This node is disabled and will not be called.\nDrag off pins to build functionality.
)

(event Collision|EventActorBeginOverlap
  (params (OtherActor :type Actor%20Object%20Reference))
  ;[1 1 1] TODO find a way to check if exit is connected (this probably doesnt work beacause exits have collision disabled after connecting)
  (Utilities|Casting|CastToBP_Exit OtherActor)
  (Development|PrintString "overlap with other exit")
  (Variables|Default|SetbIsConnected true)
  (|CallParentFunction OtherActor))

(event EventTick
  (params (DeltaSeconds :type Float%20%28single-precision%29))
  (|CallParentFunction DeltaSeconds) ; This node is disabled and will not be called.\nDrag off pins to build functionality.
)

(fn ConstructionScript
  (|CallParentFunction))

(fn IsConnected
  (return (Variables|Default|GetbIsConnected)))