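; Map tile actor for DiceRuler's map generation, with a ghost state marked by a building decal.
; On BeginPlay it spawns exits or walls at brick-mesh sockets from MapFragmentInfo, plus encounters at floor sockets and two move fields.
; While a ghost in Map Generation input mode, it cursor-traces each tick to highlight its exits; selecting one clears the ghost state.
; Helpers report unconnected exits and toggle exit collision; move-field highlighting is unfinished.
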(event EventTick
  (params (DeltaSeconds :type Float%20%28single-precision%29))
  (switch Utilities|FlowControl|Switch|SwitchonE_InputMode (CallFunction|GetCurrentInputMode)
    (:NewEnumerator1
      (CallFunction|HighlightExit))))

(event Collision|EventActorBeginOverlap
  (params (OtherActor :type Actor%20Object%20Reference)))

(event EventBeginPlay
  (CallFunction|InitExits)
  (CallFunction|InitWalls)
  (CallFunction|ShowBuildingDecal (Variables|Default|GetIsGhost))
  (CallFunction|InitEncounters)
  (CallFunction|InitMoveFields))

(fn ConstructionScript)

(fn InitEncounters
  (bind _mapfragmentinfo (Variables|Default|GetMapFragmentInfo))
  (bind (_isstartingfragment _exits _encounters) (Utilities|Struct|BreakS_MapFragment _mapfragmentinfo))
  (if (> (Utilities|Array|Length _exits) 0)
    (for (_ _array_index) (Variables|Default|GetExitObjs)
      (if (> (Utilities|Array|Length _encounters) 0)
        (if (Utilities|Array|Get(acopy) _encounters _array_index)
          (bind _returnvalue (Game|SpawnActorfromClass "/Game/DiceRuler/MapGeneration/BP_Encounter.BP_Encounter_C" (Math|Transform|MakeTransform (+ (.Location (Math|Transform|BreakTransform (Transformation|GetSocketTransform (Variables|Default|GetSM_WoodFloor) (Utilities|Array|Get(acopy) (Variables|Default|GetSocketNames) _array_index) "RTS_World"))) "0.000000,0.000000,30.000000") (.Rotation (Math|Transform|BreakTransform (Transformation|GetSocketTransform (Variables|Default|GetSM_WoodFloor) (Utilities|Array|Get(acopy) (Variables|Default|GetSocketNames) _array_index) "RTS_World"))) (.Scale (Math|Transform|BreakTransform (Transformation|GetSocketTransform (Variables|Default|GetSM_WoodFloor) (Utilities|Array|Get(acopy) (Variables|Default|GetSocketNames) _array_index) "RTS_World")))) "Undefined" "MultiplyWithRoot" 0 0))
          (Utilities|Array|Add (Variables|Default|GetEncounters) _returnvalue))))))

(fn InitExits
  (bind _sm_brick (Variables|Default|GetSM_Brick))
  (Utilities|Array|Clear (Variables|Default|GetExitObjs))
  (for (_array_element _array_index) (.Exits (Utilities|Struct|BreakS_MapFragment (Variables|Default|GetMapFragmentInfo)))
    (if _array_element
      (bind _returnvalue (Game|SpawnActorfromClass "/Game/DiceRuler/MapGeneration/BP_Exit.BP_Exit_C" (Transformation|GetSocketTransform _sm_brick (Utilities|Array|Get(acopy) (Transformation|GetAllSocketNames _sm_brick) _array_index) "RTS_World") "Undefined" "MultiplyWithRoot" 0 self (Utilities|Array|Get(acopy) (Transformation|GetAllSocketNames _sm_brick) _array_index) 0))
      (Transformation|AttachActorToActor _returnvalue self (Utilities|Array|Get(acopy) (Transformation|GetAllSocketNames _sm_brick) _array_index) "KeepWorld" "KeepWorld" "KeepRelative" true)
      (Utilities|Array|Add (Variables|Default|GetExitObjs) _returnvalue))))

(fn InitWalls
  (bind _sm_brick (Variables|Default|GetSM_Brick))
  (for (_array_element _array_index) (.Exits (Utilities|Struct|BreakS_MapFragment (Variables|Default|GetMapFragmentInfo)))
    (if (not _array_element)
      (bind _returnvalue (Game|SpawnActorfromClass "/Game/DiceRuler/MapGeneration/BP_Wall.BP_Wall_C" (Transformation|GetSocketTransform _sm_brick (Utilities|Array|Get(acopy) (Transformation|GetAllSocketNames _sm_brick) _array_index) "RTS_World") "Undefined" "MultiplyWithRoot" 0 self (Utilities|Array|Get(acopy) (Transformation|GetAllSocketNames _sm_brick) _array_index) 0))
      (Transformation|AttachActorToActor _returnvalue self (Utilities|Array|Get(acopy) (Transformation|GetAllSocketNames _sm_brick) _array_index) "KeepWorld" "KeepWorld" "KeepRelative" true))))

(fn InitMoveFields
  (bind _output_get (LocalVariables|SetSpawnPoints (Utilities|Array|MakeArray (Variables|Default|GetSpawnPointMoveField1) (Variables|Default|GetSpawnPointMoveField2))))
  (for _array_element _output_get
    (bind _returnvalue (Game|SpawnActorfromClass "/Game/DiceRuler/MapGeneration/BP_MoveField.BP_MoveField_C" (Transformation|GetWorldTransform _array_element) "Undefined" "MultiplyWithRoot" 0 0 "None" 0))
    (Transformation|AttachActorToActor _returnvalue self "None" "KeepWorld" "KeepWorld" "KeepRelative" true)))

(fn ShowBuildingDecal
  (params (IsShown :type Boolean))
  (Rendering|SetVisibility (Variables|Default|GetDecal) IsShown false)
  (Variables|Default|SetIsGhost IsShown))

(fn SelectExit
  (params (ExitHit :type BP%20Exit%20Object%20Reference))
  (if (Variables|Default|GetIsGhost)
    (if (Utilities|Array|ContainsItem (Variables|Default|GetExitObjs) ExitHit)
      (if (== (Variables|Default|GetSelectedExit) ExitHit)
        _
        (else
          (Utilities|IsValid (Variables|Default|GetSelectedExit)
            (:Is%20Valid
              (Default|SetSelected (Variables|Default|GetSelectedExit) false))
            (:Is%20Not%20Valid
              _))
          (Variables|Default|SetSelectedExit ExitHit)
          (Default|SetSelected ExitHit true)
          (CallFunction|ShowBuildingDecal false)
          (return ExitHit))))
    (return (Variables|Default|GetSelectedExit))))

(fn CheckActorUnderCursor
  (bind _returnvalue (Game|GetPlayerController 0))
  (bind (_hitresult _returnvalue_2) (Game|Player|GetHitResultUnderCursorbyChannel _returnvalue "TraceTypeQuery1" true))
  (if _returnvalue_2
    (return (.HitActor (Collision|BreakHitResult _hitresult)))
    (else
      (return 0))))

(fn HighlightExit
  (if (Variables|Default|GetIsGhost)
    (bind _actorundercursor (CallFunction|CheckActorUnderCursor))
    (bind _asbp_exit (Utilities|Casting|CastToBP_Exit _actorundercursor)
      (:then
        (if (Utilities|Array|ContainsItem (Variables|Default|GetExitObjs) _asbp_exit)
          (if (== (Variables|Default|GetHighlightedExit) 0)
            (Default|SetHighlight _asbp_exit "NewEnumerator1")
            (Variables|Default|SetHighlightedExit _asbp_exit)
            (elif (not (== (Variables|Default|GetHighlightedExit) (Variables|Default|GetSelectedExit)))
              (if (not (== _asbp_exit (Variables|Default|GetSelectedExit)))
                (if (not (== (Variables|Default|GetHighlightedExit) _asbp_exit))
                  (Default|SetHighlight (Variables|Default|GetHighlightedExit) "NewEnumerator0")
                  (Default|SetHighlight _asbp_exit "NewEnumerator1")
                  (Variables|Default|SetHighlightedExit _asbp_exit)))))))
      (:CastFailed
        (Utilities|IsValid (Variables|Default|GetHighlightedExit)
          (:Is%20Valid
            (if (not (== (Variables|Default|GetSelectedExit) (Variables|Default|GetHighlightedExit)))
              (Default|SetHighlight (Variables|Default|GetHighlightedExit) "NewEnumerator0")
              (Variables|Default|SetHighlightedExit 0))))))))

(fn HighlightMoveField
  (bind _actorundercursor (CallFunction|CheckActorUnderCursor))
  (bind _asbp_move_field (Utilities|Casting|CastToBP_MoveField _actorundercursor)))

(fn FindUnConnectedExits
  (for _array_element (Variables|Default|GetExitObjs)
    (bind _outisconnected (Default|IsConnected _array_element))
    (if (not _outisconnected)
      (Utilities|Array|Add (LocalVariables|GetUnConnectedExits) _array_element)))
  (return (LocalVariables|GetUnConnectedExits)))

(fn SetCollsionEnableinExits
  (params (bNewActorEnableCollision :type Boolean))
  (for _array_element (Variables|Default|GetExitObjs)
    (Collision|SetActorEnableCollision _array_element bNewActorEnableCollision)))