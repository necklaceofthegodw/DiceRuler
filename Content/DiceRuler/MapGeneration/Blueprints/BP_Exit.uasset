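; BP_Exit is an exit on a generated map fragment that shows whether the way is locked, open or connected.
; On BeginPlay, connected exits drop ExitBlock collision, while unconnected ones keep it and show locked if their parent is an unfinished puzzle fragment.
; SetExitState stores the state and swaps the block's material, falling back to a wall material.
; SetIsConnected updates flag and state but leaves collision unchanged.
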(event EventBeginPlay
  (bind _exitblock (Variables|Default|GetExitBlock))
  (|CallParentFunction)
  (if (Variables|Default|GetbIsConnected)
    (Collision|SetCollisionEnabled _exitblock "NoCollision")
    (CallFunction|SetExitState "NewEnumerator2")
    (else
      (Collision|SetCollisionEnabled _exitblock "QueryAndPhysics")
      (bind _asbp_puzzle_map_fragment (Utilities|Casting|CastToBP_PuzzleMapFragment (Variables|Default|GetParentMapFragment))
        (:then
          (if (Variables|/Game/DiceRuler/MapGeneration/Blueprints/BP_PuzzleMapFragment.BP_PuzzleMapFragment_C|GetPuzzleFinished? _asbp_puzzle_map_fragment)
            (CallFunction|SetExitState "NewEnumerator1" :!label _label)
            (else
              (CallFunction|SetExitState "NewEnumerator0"))))
        (:CastFailed
          (goto _label))))))

(event EventTick
  (params (DeltaSeconds :type Float%20%28single-precision%29))
  (|CallParentFunction DeltaSeconds) ; This node is disabled and will not be called.\nDrag off pins to build functionality.
)

(fn ConstructionScript
  (|CallParentFunction))

(fn IsConnected
  (return (Variables|Default|GetbIsConnected)))

(fn SetIsConnected
  (params (IsConnectedToSet :type Boolean))
  (Variables|Default|SetbIsConnected IsConnectedToSet)
  (CallFunction|SetExitState "NewEnumerator2"))

(fn SetExitVisible
  (params (IsVisible :type Boolean))
  (Development|SetHiddeninGame (Variables|Default|GetExitBlock) (not IsVisible) false))

(fn SetExitState
  (params (stateToSet :type E_ExitState%20Enum :default "NewEnumerator0"))
  (bind _output_get (Variables|Default|SetCurrentState stateToSet))
  (switch Utilities|FlowControl|Switch|SwitchonE_ExitState _output_get
    (:NewEnumerator0
      (LocalVariables|SetCurrentMaterial (Variables|Default|GetMaterialLocked)))
    (:NewEnumerator1
      (LocalVariables|SetCurrentMaterial (Variables|Default|GetMaterialUnlockedNotConnected)))
    (:NewEnumerator2
      (LocalVariables|SetCurrentMaterial (Variables|Default|GetMaterialUnlockedConnected)))
    (:NewEnumerator3
      (LocalVariables|SetCurrentMaterial (Variables|Default|GetMaterialWall))))
  (Rendering|Material|SetMaterial (Variables|Default|GetExitBlock) 0 (LocalVariables|GetCurrentMaterial)))