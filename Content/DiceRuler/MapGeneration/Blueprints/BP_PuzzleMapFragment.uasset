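; BP_PuzzleMapFragment is a map fragment that hosts a puzzle the dice player starts by stepping into a trigger.
; The first overlap sets it as the player's active puzzle, and spawning optionally rotates the trigger and puzzle spawn point.
; Finishing spawns a rune reward above the trigger, hides the trigger, saves completion through the game instance, shows the move-choice HUD and updates unconnected exits' state.
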(event OnComponentBeginOverlap(StartPuzzleTrigger2)
  (params (OverlappedComponent :type Primitive%20Component%20Object%20Reference) (OtherActor :type Actor%20Object%20Reference) (OtherComp :type Primitive%20Component%20Object%20Reference) (OtherBodyIndex :type Integer) (bFromSweep :type Boolean) (SweepResult :type Hit%20Result%20Structure%20%28by%20ref%29))
  (bind _asbp_dice_player_character (Utilities|Casting|CastToBP_DicePlayerCharacter OtherActor))
  (if (not (Variables|Default|GetPuzzleStarted?))
    (Variables|Default|SetPuzzleStarted? true)
    (Default|SetActivePuzzle _asbp_dice_player_character self)
    (Puzzle|PuzzleTriggered)))

(event EventBeginPlay
  (|CallParentFunction) ; This node is disabled and will not be called.\nDrag off pins to build functionality.
)

(event Collision|EventActorBeginOverlap
  (params (OtherActor :type Actor%20Object%20Reference)))

(event EventTick
  (params (DeltaSeconds :type Float%20%28single-precision%29))
  (|CallParentFunction DeltaSeconds) ; This node is disabled and will not be called.\nDrag off pins to build functionality.
)

(fn ConstructionScript
  (|CallParentFunction))

(fn RotatePuzzleifNeeded0
  (bind _brotatepuzzleonspawn (Variables|Default|GetbRotatePuzzleOnSpawn))
  (Transformation|SetRelativeTransform (Variables|Default|GetStartPuzzleTrigger2) (Math|Transform|SelectTransform (LocalVariables|GetTriggerTransformRotated) (LocalVariables|GetTriggerTransformInitial) _brotatepuzzleonspawn) false false)
  (Transformation|SetRelativeRotation (Variables|Default|GetSM_PuzzleSpawnTransform2) (Math|Rotator|SelectRotator "0.000000,180.000000,0.000000" "0, 0, 0" _brotatepuzzleonspawn) false false))

(fn SpawnPuzzle
  (|CallParentFunction)
  (CallFunction|RotatePuzzleifNeeded0))

(fn SpawnReward
  (bind _startpuzzletrigger2 (Variables|Default|GetStartPuzzleTrigger2))
  (bind _returnvalue (Transformation|GetWorldLocation _startpuzzletrigger2))
  (bind (_x _y _z) (Math|Vector|BreakVector _returnvalue))
  (Game|SpawnActorfromClass "/Game/DiceRuler/Puzzles/Memory/BP_RuneReward.BP_RuneReward_C" (Math|Transform|MakeTransform (Math|Vector|MakeVectorNetQuantize _x _y (+ _z 3e+02))) "Undefined" "MultiplyWithRoot" 0 0 0))

(fn PuzzleFinished
  (|CallParentFunction)
  (Variables|Default|SetPuzzleFinished? true)
  (CallFunction|SpawnReward)
  (CallFunction|HidePuzzleTrigger)
  (Variables|Default|SetMapFragmentInfo (Utilities|Struct|MakeS_MapFragment (.IsStartingFragment (Utilities|Struct|BreakS_MapFragment (Variables|Default|GetMapFragmentInfo))) (.Exits (Utilities|Struct|BreakS_MapFragment (Variables|Default|GetMapFragmentInfo))) (.ExitsThatAreConnected (Utilities|Struct|BreakS_MapFragment (Variables|Default|GetMapFragmentInfo))) (Transformation|GetActorTransform) true (.MapFragmentClass (Utilities|Struct|BreakS_MapFragment (Variables|Default|GetMapFragmentInfo)))))
  (Default|UpdateMapFragmentDatainSave (CallFunction|GetDiceRulerGameInstance) (Variables|Default|GetIndex) (Utilities|Struct|MakeS_MapFragment (.IsStartingFragment (Utilities|Struct|BreakS_MapFragment (Variables|Default|GetMapFragmentInfo))) (.Exits (Utilities|Struct|BreakS_MapFragment (Variables|Default|GetMapFragmentInfo))) (.ExitsThatAreConnected (Utilities|Struct|BreakS_MapFragment (Variables|Default|GetMapFragmentInfo))) (Transformation|GetActorTransform) true (.MapFragmentClass (Utilities|Struct|BreakS_MapFragment (Variables|Default|GetMapFragmentInfo)))))
  (Default|ShowChooseMove (CallFunction|GetDiceHud) true)
  (for _array_element (Variables|Default|GetExitObjs)
    (bind _outisconnected (Default|IsConnected _array_element))
    (if (not _outisconnected)
      (Default|SetExitState _array_element "NewEnumerator1"))))

(fn PuzzleTriggered)

(fn HidePuzzleTrigger
  (bind _startpuzzletrigger2 (Variables|Default|GetStartPuzzleTrigger2))
  (Development|SetHiddeninGame _startpuzzletrigger2 true false)
  (Collision|SetCollisionEnabled _startpuzzletrigger2 "NoCollision")
  (Development|SetHiddeninGame (Variables|Default|GetNiagara1) true false))