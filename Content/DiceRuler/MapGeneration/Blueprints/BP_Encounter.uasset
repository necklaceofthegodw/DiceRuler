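; BP_Encounter is an encounter marker actor with a Point Light and a sphere trigger, part of the map generation system.
; On BeginPlay its IsHalf flag sets the light to a dim gold, or to a much brighter red for full encounters.
; When the top-down character enters the sphere of a non-half encounter, it only prints a debug message.
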(event OnComponentBeginOverlap(Sphere)
  (params (OverlappedComponent :type Primitive%20Component%20Object%20Reference) (OtherActor :type Actor%20Object%20Reference) (OtherComp :type Primitive%20Component%20Object%20Reference) (OtherBodyIndex :type Integer) (bFromSweep :type Boolean) (SweepResult :type Hit%20Result%20Structure%20%28by%20ref%29))
  (if (not (Variables|Default|GetIsHalf))
    (Utilities|Casting|CastToBP_TopDownCharacter OtherActor)
    (Development|PrintString "player overlap with encounter")))

(event EventBeginPlay
  (bind _pointlight (Variables|Default|GetPointLight))
  (if (Variables|Default|GetIsHalf)
    (Rendering|Components|Light|SetLightColor _pointlight "(R=0.765625,G=0.595282,B=0.105796,A=1.000000)" true)
    (Rendering|Components|Light|SetIntensity _pointlight 5e+02)
    (else
      (Rendering|Components|Light|SetLightColor _pointlight "(R=0.927083,G=0.053114,B=0.101581,A=1.000000)" true)
      (Rendering|Components|Light|SetIntensity _pointlight 5e+03))))

(event Collision|EventActorBeginOverlap
  (params (OtherActor :type Actor%20Object%20Reference)))

(event EventTick
  (params (DeltaSeconds :type Float%20%28single-precision%29)))

(fn ConstructionScript)