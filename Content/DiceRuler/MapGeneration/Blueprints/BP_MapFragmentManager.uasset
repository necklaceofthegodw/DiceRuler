(event Custom|SpawnPuzzleDelayed
  (params (MapFragment :type BP%20Map%20Fragment%20Object%20Reference))
  (Utilities|FlowControl|Delay 2.0)
  (Default|SpawnPuzzle MapFragment))

(event EventBeginPlay
  (bind _asbp_dice_ruler_game_instance (CallFunction|GetDiceRulerGameInstance))
  (bind _returnvalue (SaveGame|DoesSaveGameExist (Variables|/Game/DiceRuler/BP_DiceRulerGameInstance.BP_DiceRulerGameInstance_C|GetSavedGameSlotName _asbp_dice_ruler_game_instance)))
  (if _returnvalue
    (bind (_spawnedfragments _levelspipe _levelssokoban) (Default|RecreateMapFragments _asbp_dice_ruler_game_instance))
    (bind _output_get (Variables|Default|SetSpawnedMapFragments _spawnedfragments))
    (Variables|levels|SetLevelsPipe _levelspipe)
    (Variables|Levels|SetLevelsSokoban _levelssokoban)
    (Variables|Default|SetFirstMapFragment (Utilities|Array|Get(acopy) _output_get))
    (else
      (levels|SetAvailableLevelsPipePuzzle)
      (levels|SetAvailableLevelsSokobanPuzzle)
      (CallFunction|SpawnFirstMapFragment))))

(event Collision|EventActorBeginOverlap
  (params (OtherActor :type Actor%20Object%20Reference)))

(event EventTick
  (params (DeltaSeconds :type Float%20%28single-precision%29)))

(fn ConstructionScript)

(fn SpawnFirstMapFragment
  (bind _outtransform (CallFunction|GetDicePlayerStartPosition))
  (bind _map_fragment_info (Variables|Default|GetMap%20Fragment%20Info))
  (bind (_isstartingfragment _exits _exitsthatareconnected) (Utilities|Struct|BreakS_MapFragment _map_fragment_info))
  (bind (_location _rotation _scale) (Math|Transform|BreakTransform _outtransform))
  (bind _returnvalue (- _location "700.000000,700.000000,0.000000"))
  (bind _returnvalue_2 (Math|Transform|MakeTransform _returnvalue _rotation _scale))
  (bind _returnvalue_3 (Game|SpawnActorfromClass "/Game/DiceRuler/MapGeneration/Blueprints/BP_MapFragment.BP_MapFragment_C" _returnvalue_2 "Undefined" "MultiplyWithRoot" 0 (Variables|Default|GetMap%20Fragment%20Info) false 0))
  (bind _output_get (Variables|Default|SetFirstMapFragment _returnvalue_3))
  (Utilities|Array|Add (Variables|Default|GetSpawnedMapFragments) _output_get)
  (Default|AddMapFragmentDatatoSave (CallFunction|GetDiceRulerGameInstance) (Utilities|Struct|MakeS_MapFragment _isstartingfragment _exits _exitsthatareconnected _returnvalue_2) (Variables|levels|GetLevelsPipe) (Variables|Levels|GetLevelsSokoban)))

(fn SpawnMapFragment
  (bind _outmapfragment (CallFunction|GetDicePlayerMapFragment))
  (bind _output_get (Variables|Default|SetPlayerMapFragment _outmapfragment))
  (bind _outspawnlocation (CallFunction|ChecktoSpawnontheOtherSide _output_get))
  (LocalVariables|SetSpawnOffset _outspawnlocation)
  (bind _output_get_2 (LocalVariables|SetCurrentExitConfig (Utilities|Select :Index (Math|Random|RandomIntegerinRange 0 4) :Option%200 (LocalVariables|GetExitsConfig) :Option%201 (LocalVariables|GetExitsConfig_0) :Option%202 (LocalVariables|GetExitsConfig_1) :Option%203 (LocalVariables|GetExitsConfig_2) :Option%204 (LocalVariables|GetExitsConfig_3))))
  ;[1 1 1] Add encounter to the second existing exit
  (for (_array_element _array_index) _output_get_2
    (if _array_element
      (if (LocalVariables|GetFirstExistingExit)
        (Utilities|Array|SetArrayElem (LocalVariables|GetEncounters) _array_index true)
        (else
          (LocalVariables|SetFirstExistingExit true)))))
  (bind _returnvalue (Game|SpawnActorfromClass (.OutItem (Utilities|Array|Random (Variables|Default|GetMapFragmentClassesToSpawn))) (Math|Transform|MakeTransform (+ (.Origin (Collision|GetActorBounds (Variables|Default|GetPlayerMapFragment) false false)) (LocalVariables|GetSpawnOffset))) "Undefined" "MultiplyWithRoot" 0 (Utilities|Struct|MakeS_MapFragment false (LocalVariables|GetCurrentExitConfig) (Utilities|Array|MakeArray false false false false false false) (Math|Transform|MakeTransform (+ (.Origin (Collision|GetActorBounds (Variables|Default|GetPlayerMapFragment) false false)) (LocalVariables|GetSpawnOffset)))) true 0))
  (bind _output_get_3 (Variables|Default|SetCurrentlySpawnedFragment _returnvalue))
  (Utilities|Array|Add (Variables|Default|GetSpawnedMapFragments) _output_get_3)
  (CallFunction|SetWallsVisibilityinAllMapFragments false))

(fn TrySelectExit
  (params (PlayerController :type Player%20Controller%20Object%20Reference))
  (bind _playermapfragment (Variables|Default|GetPlayerMapFragment))
  (bind _playermapfragment_2 (Variables|Default|GetPlayerMapFragment))
  (bind _currentlyspawnedfragment (Variables|Default|GetCurrentlySpawnedFragment))
  (bind _asbp_exit (Utilities|Casting|CastToBP_Exit (.HitActor (Collision|BreakHitResult (.HitResult (Game|Player|GetHitResultUnderCursorbyChannel PlayerController "TraceTypeQuery1" true))))))
  (Utilities|IsValid (Variables|Default|GetFirstSelectedExit)
    (:Is%20Valid
      (Utilities|IsValid _playermapfragment
        (:Is%20Valid
          (bind _outselectedexit (Default|SelectExit _playermapfragment _asbp_exit))
          (Variables|Default|SetSecondSelectedExit _outselectedexit)
          (CallFunction|ConnectMapFragments))))
    (:Is%20Not%20Valid
      (Utilities|IsValid _currentlyspawnedfragment
        (:Is%20Valid
          (bind _outselectedexit_2 (Default|SelectExit _currentlyspawnedfragment _asbp_exit))
          (bind _output_get (Variables|Default|SetFirstSelectedExit _outselectedexit_2))
          (Default|ShowBuildingDecal (Variables|/Game/DiceRuler/MapGeneration/Blueprints/BP_SelectableObject.BP_SelectableObject_C|GetParentMapFragment _output_get) false)
          (Default|SetRotatePuzzleonSpawn (Variables|/Game/DiceRuler/MapGeneration/Blueprints/BP_SelectableObject.BP_SelectableObject_C|GetParentMapFragment _output_get))
          (Utilities|IsValid _playermapfragment_2
            (:Is%20Valid
              (Default|ShowBuildingDecal _playermapfragment_2 true))))))))

(fn ChecktoSpawnNextFragment
  (bind _playermapfragment (Variables|Default|GetPlayerMapFragment))
  (Utilities|IsValid (Variables|Default|GetFirstSelectedExit)
    (:Is%20Valid
      (Utilities|IsValid (Variables|Default|GetSecondSelectedExit)
        (:Is%20Valid
          (Math|Integer|IncrementInt (Variables|Default|GetSpawnedFragmentsCount)
            (:%20%20
              (if (CallFunction|AreMapFragmentsColliding)
                (Development|PrintString "fragments are colliding, choose other exit or exit build mode")
                (else
                  (CallFunction|FinishConnectingMapFragments)
                  (if (== (Variables|Default|GetSpawnedFragmentsCount) 3)
                    (Input|ExitBuildMode false :!label _label)
                    (Variables|Default|SetSpawnedFragmentsCount 0)
                    (else
                      (bind _outunconnectedexits (Default|FindUnConnectedExits (Variables|Default|GetPlayerMapFragment)))
                      (if (> (Utilities|Array|Length _outunconnectedexits) 0)
                        (Variables|Default|SetFirstSelectedExit 0)
                        (Variables|Default|SetSecondSelectedExit 0)
                        (Variables|/Game/DiceRuler/MapGeneration/Blueprints/BP_MapFragment.BP_MapFragment_C|SetHighlightedExit _playermapfragment 0)
                        (Variables|/Game/DiceRuler/MapGeneration/Blueprints/BP_MapFragment.BP_MapFragment_C|SetSelectedExit _playermapfragment 0)
                        (Variables|Default|SetSpawnedFragmentsCount 0)
                        (CallFunction|SpawnMapFragment)
                        (else
                          (goto _label))))))))))
        (:Is%20Not%20Valid
          (Development|PrintString "select exit first" :!label _label_2))))
    (:Is%20Not%20Valid
      (goto _label_2))))

(fn ConnectMapFragments
  (bind _firstselectedexit (Variables|Default|GetFirstSelectedExit))
  (bind _secondselectedexit (Variables|Default|GetSecondSelectedExit))
  (bind _firstselectedexit_2 (Variables|Default|GetFirstSelectedExit))
  (bind _parentmapfragment (Variables|/Game/DiceRuler/MapGeneration/Blueprints/BP_SelectableObject.BP_SelectableObject_C|GetParentMapFragment _firstselectedexit))
  (if (and (Utilities|IsValid (Variables|Default|GetFirstSelectedExit)) (Utilities|IsValid (Variables|Default|GetSecondSelectedExit)))
    (LocalVariables|SetSelectedExit_AndRotations (Utilities|Select :Index (Utilities|Array|FindItem (Transformation|GetAllSocketNames (Variables|/Game/DiceRuler/MapGeneration/Blueprints/BP_MapFragment.BP_MapFragment_C|GetSM_Brick (Variables|/Game/DiceRuler/MapGeneration/Blueprints/BP_SelectableObject.BP_SelectableObject_C|GetParentMapFragment _firstselectedexit_2))) (Variables|/Game/DiceRuler/MapGeneration/Blueprints/BP_SelectableObject.BP_SelectableObject_C|GetAttachSocketName _firstselectedexit_2)) :Option%200 (LocalVariables|GetSocketExit_0_AndRotations) :Option%201 (LocalVariables|GetSocketExit_1_AndRotations) :Option%202 (LocalVariables|GetSocketExit_2_AndRotations) :Option%203 (LocalVariables|GetSocketExit_3_AndRotations) :Option%204 (LocalVariables|GetSocketExit_4_AndRotations) :Option%205 (LocalVariables|GetSocketExit_5_AndRotations)))
    (Transformation|SetActorRotation _parentmapfragment (Math|Rotator|CombineRotators (Transformation|GetActorRotation (Variables|/Game/DiceRuler/MapGeneration/Blueprints/BP_SelectableObject.BP_SelectableObject_C|GetParentMapFragment _secondselectedexit)) (.Value (Utilities|Map|Find (LocalVariables|GetSelectedExit_AndRotations) (Variables|/Game/DiceRuler/MapGeneration/Blueprints/BP_SelectableObject.BP_SelectableObject_C|GetAttachSocketName _secondselectedexit)))))
    (Transformation|SetActorLocation _parentmapfragment (+ (Transformation|GetActorLocation _secondselectedexit) (- (Transformation|GetActorLocation _parentmapfragment) (Transformation|GetActorLocation _firstselectedexit))) false false)
    (else
      (Development|PrintString "try connecting exits not selected"))))

(fn FinishConnectingMapFragments
  (bind _asbp_dice_ruler_game_instance (CallFunction|GetDiceRulerGameInstance))
  (bind _firstselectedexit (Variables|Default|GetFirstSelectedExit))
  (bind _secondselectedexit (Variables|Default|GetSecondSelectedExit))
  (bind _firstselectedexit_2 (Variables|Default|GetFirstSelectedExit))
  (bind _firstselectedexit_3 (Variables|Default|GetFirstSelectedExit))
  (bind _parentmapfragment (Variables|/Game/DiceRuler/MapGeneration/Blueprints/BP_SelectableObject.BP_SelectableObject_C|GetParentMapFragment _firstselectedexit))
  (bind _parentmapfragment_2 (Variables|/Game/DiceRuler/MapGeneration/Blueprints/BP_SelectableObject.BP_SelectableObject_C|GetParentMapFragment _firstselectedexit_2))
  (bind _mapfragmentinfo (Variables|/Game/DiceRuler/MapGeneration/Blueprints/BP_MapFragment.BP_MapFragment_C|GetMapFragmentInfo _parentmapfragment_2))
  (bind (_isstartingfragment _exits _exitsthatareconnected) (Utilities|Struct|BreakS_MapFragment _mapfragmentinfo))
  (if (and (Utilities|IsValid (Variables|Default|GetFirstSelectedExit)) (Utilities|IsValid (Variables|Default|GetSecondSelectedExit)))
    (Variables|Default|SetbCanExitBuildingmode true)
    (Default|SetHighlight (Variables|Default|GetFirstSelectedExit) "NewEnumerator0")
    (bind _asbp_exit (Utilities|Casting|CastToBP_Exit _firstselectedexit_3))
    (Default|SetIsConnected _asbp_exit true)
    (Default|SetConnectedExits (Variables|/Game/DiceRuler/MapGeneration/Blueprints/BP_SelectableObject.BP_SelectableObject_C|GetParentMapFragment _firstselectedexit_3) _asbp_exit)
    (bind _asbp_exit_2 (Utilities|Casting|CastToBP_Exit _secondselectedexit))
    (Default|SetIsConnected _asbp_exit_2 true)
    (Default|SetConnectedExits (Variables|/Game/DiceRuler/MapGeneration/Blueprints/BP_SelectableObject.BP_SelectableObject_C|GetParentMapFragment _secondselectedexit) _asbp_exit_2)
    (Default|SetCollsionEnableinExits _parentmapfragment)
    (Collision|SetActorEnableCollision (Variables|Default|GetSecondSelectedExit) false)
    (Default|ShowPreview _parentmapfragment false)
    (Default|SpawnPuzzle _parentmapfragment)
    (Default|ShowBuildingDecal (Variables|/Game/DiceRuler/MapGeneration/Blueprints/BP_SelectableObject.BP_SelectableObject_C|GetParentMapFragment (Variables|Default|GetSecondSelectedExit)) false)
    (if (Variables|/Game/DiceRuler/BP_DiceRulerGameInstance.BP_DiceRulerGameInstance_C|GetbIsGameSaved _asbp_dice_ruler_game_instance)
      (Default|AddMapFragmentDatatoSave _asbp_dice_ruler_game_instance (Utilities|Struct|MakeS_MapFragment _isstartingfragment _exits _exitsthatareconnected (Transformation|GetActorTransform _parentmapfragment_2)) (Variables|levels|GetLevelsPipe) (Variables|Levels|GetLevelsSokoban)))
    (else
      (Development|PrintString "Finish connecting exits not selected"))))

(fn ChecktoSpawnontheOtherSide
  (params (MapFragmentToCheck :type BP%20Map%20Fragment%20Object%20Reference))
  (return (Math|Vector|SelectVector (LocalVariables|GetSpawnOffsetLeft) (LocalVariables|GetSpawnOffsetRight) (== (.Yaw (Math|Rotator|BreakRotator (Transformation|GetActorRotation MapFragmentToCheck))) -9e+01))))

(fn ExitBuildMode
  (params (IsExitForced :type Boolean))
  (bind _playermapfragment (Variables|Default|GetPlayerMapFragment))
  (if (Variables|Default|GetbCanExitBuildingmode)
    (if IsExitForced
      (Utilities|Array|RemoveItem (Variables|Default|GetSpawnedMapFragments) (Variables|Default|GetCurrentlySpawnedFragment))
      (Default|DeleteExits (Variables|Default|GetCurrentlySpawnedFragment))
      (Actor|DestroyActor (Variables|Default|GetCurrentlySpawnedFragment)))
    (Variables|Default|SetCurrentlySpawnedFragment 0)
    (Default|ChangeInputMode (CallFunction|GetDiceRulerGameInstance) "NewEnumerator0")
    (Default|ResetCameraPosition (CallFunction|GetDicePlayerCharacter))
    (Default|ShowExploreMenuWidget (Variables|/Game/DiceRuler/HUD/BP_DiceRulerHUD.BP_DiceRulerHUD_C|GetWBP_HUD (CallFunction|GetDiceHud)) false)
    (for _array_element (Variables|Default|GetSpawnedMapFragments)
      (Default|ShowBuildingDecal _array_element false))
    (Default|ShowBuildingDecal (Variables|Default|GetPlayerMapFragment) false)
    (Utilities|IsValid (Variables|Default|GetFirstSelectedExit)
      (:Is%20Valid
        (Default|SetHighlight (Variables|Default|GetFirstSelectedExit) "NewEnumerator0")
        (Variables|Default|SetFirstSelectedExit 0))
      (:Is%20Not%20Valid
        _))
    (Utilities|IsValid (Variables|Default|GetSecondSelectedExit)
      (:Is%20Valid
        (Default|SetHighlight (Variables|Default|GetSecondSelectedExit) "NewEnumerator0")
        (Variables|Default|SetSecondSelectedExit 0))
      (:Is%20Not%20Valid
        _))
    (Variables|/Game/DiceRuler/MapGeneration/Blueprints/BP_MapFragment.BP_MapFragment_C|SetHighlightedExit _playermapfragment 0)
    (Variables|/Game/DiceRuler/MapGeneration/Blueprints/BP_MapFragment.BP_MapFragment_C|SetSelectedExit _playermapfragment 0)
    (CallFunction|SetWallsVisibilityinAllMapFragments true)
    (Default|CallBuildModeClosed)
    (else
      (Development|PrintString "finish connecting before exiting build mode"))))

(fn SetWallsVisibilityinAllMapFragments
  (params (IsVisible :type Boolean))
  (for _array_element (Variables|Default|GetSpawnedMapFragments)
    (Default|SetWallsVisible _array_element IsVisible))
  (Default|SetWallsVisible (Variables|Default|GetFirstMapFragment) IsVisible))

(fn AreMapFragmentsColliding
  (return (or (Variables|/Game/DiceRuler/MapGeneration/Blueprints/BP_MapFragment.BP_MapFragment_C|GetIsColliding (Variables|/Game/DiceRuler/MapGeneration/Blueprints/BP_SelectableObject.BP_SelectableObject_C|GetParentMapFragment (Variables|Default|GetFirstSelectedExit))) (Variables|/Game/DiceRuler/MapGeneration/Blueprints/BP_MapFragment.BP_MapFragment_C|GetIsColliding (Variables|/Game/DiceRuler/MapGeneration/Blueprints/BP_SelectableObject.BP_SelectableObject_C|GetParentMapFragment (Variables|Default|GetSecondSelectedExit))))))

(fn GetRandomAvailableLevelPipesPuzzle
  (return (levels|GetRandomAvailableLevel (Variables|levels|GetLevelsPipe))))

(fn GetRandomAvailableLevelSokobanPuzzle
  (return (levels|GetRandomAvailableLevel (Variables|Levels|GetLevelsSokoban))))

(fn GetRandomAvailableLevel
  (params (Array :type Array%20of%20Names))
  (bind _returnvalue (Utilities|Array|Length Array))
  (if (> _returnvalue 0)
    (bind _output_get (LocalVariables|SetIndexToRemove (Math|Random|RandomIntegerinRange 0 (- _returnvalue 1))))
    (bind _output_get_2 (LocalVariables|SetChosenLevel (Utilities|Array|Get(acopy) Array _output_get)))
    (Utilities|Array|RemoveIndex Array _output_get)
    (return _output_get_2)
    (else
      (Development|PrintString "no more new levels")
      (return "level1"))))

(fn SetAvailableLevelsPipePuzzle
  (bind _outrownames (DataTable|GetDataTableRowNames "/Game/DiceRuler/Puzzles/Pipes/DT_PipesLevels.DT_PipesLevels"))
  (Variables|levels|SetLevelsPipe _outrownames))

(fn SetAvailableLevelsSokobanPuzzle
  (bind _outrownames (DataTable|GetDataTableRowNames "/Game/DiceRuler/Puzzles/Sokoban/Data/DT_Sokoban.DT_Sokoban"))
  (Variables|Levels|SetLevelsSokoban _outrownames))