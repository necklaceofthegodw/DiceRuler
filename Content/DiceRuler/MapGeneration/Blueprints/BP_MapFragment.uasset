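; Map tile actor for DiceRuler's map generation, built from an SMapFragment struct.
; On BeginPlay it spawns exits at brick mesh sockets, shows wall blocks where exits are absent, and attaches half-encounters linked to their exits.
; While in ghost state it shows a building decal and highlights exits under the cursor during Map Generation input; selecting one ends that state.
; Helpers gather unconnected exits, record connections in the struct, and toggle exit collision and wall visibility.
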(event EventTick
  (params (DeltaSeconds :type Float%20%28single-precision%29))
  (switch Utilities|FlowControl|Switch|SwitchonE_InputMode (CallFunction|GetCurrentInputMode)
    (:NewEnumerator1
      (CallFunction|HighlightExit))))

(event Collision|EventActorBeginOverlap
  (params (OtherActor :type Actor%20Object%20Reference)))

(event EventBeginPlay
  (CallFunction|InitExits)
  (CallFunction|InitWalls)
  (CallFunction|ShowBuildingDecal (Variables|Default|GetIsGhost))
  (CallFunction|InitEncounters))

(fn ConstructionScript)

(fn InitEncounters
  (bind _mapfragmentinfo (Variables|Default|GetMapFragmentInfo))
  (bind (_isstartingfragment _exits _exitsthatareconnected _encounters) (Utilities|Struct|BreakS_MapFragment _mapfragmentinfo))
  (if (> (Utilities|Array|Length _exits) 0)
    (for (_array_element _array_index) (Variables|Default|GetExitObjs)
      (if (> (Utilities|Array|Length _encounters) 0)
        (if (Utilities|Array|Get(acopy) _encounters _array_index)
          (bind _returnvalue (Game|SpawnActorfromClass "/Game/DiceRuler/MapGeneration/Blueprints/BP_Encounter.BP_Encounter_C" (Math|Transform|MakeTransform (+ (.Location (Math|Transform|BreakTransform (Transformation|GetSocketTransform (Variables|Default|GetSM_Brick) (Utilities|Array|Get(acopy) (Variables|Default|GetSocketNames) _array_index) "RTS_World"))) "0.000000,0.000000,30.000000") (.Rotation (Math|Transform|BreakTransform (Transformation|GetSocketTransform (Variables|Default|GetSM_Brick) (Utilities|Array|Get(acopy) (Variables|Default|GetSocketNames) _array_index) "RTS_World"))) (.Scale (Math|Transform|BreakTransform (Transformation|GetSocketTransform (Variables|Default|GetSM_Brick) (Utilities|Array|Get(acopy) (Variables|Default|GetSocketNames) _array_index) "RTS_World")))) "Undefined" "MultiplyWithRoot" 0 true 0))
          (Utilities|Array|Add (Variables|Default|GetEncounters) _returnvalue)
          (Transformation|AttachActorToActor _returnvalue self "None" "KeepWorld" "KeepWorld" "KeepWorld" true)
          (Default|SetHalfEncounter (.AsBP%20Exit (Utilities|Casting|CastToBP_Exit _array_element)) _returnvalue)
          (Default|SetHasEncounter (.AsBP%20Exit (Utilities|Casting|CastToBP_Exit _array_element)) true))))))

(fn InitExits
  (bind _sm_brick (Variables|Default|GetSM_Brick))
  (bind _mapfragmentinfo (Variables|Default|GetMapFragmentInfo))
  (bind (_isstartingfragment _exits _exitsthatareconnected _encounters) (Utilities|Struct|BreakS_MapFragment _mapfragmentinfo))
  (Utilities|Array|Clear (Variables|Default|GetExitObjs))
  (for (_array_element _array_index) _exits
    (if _array_element
      (bind _returnvalue (Game|SpawnActorfromClass "/Game/DiceRuler/MapGeneration/Blueprints/BP_Exit.BP_Exit_C" (Math|Transform|MakeTransform (.Location (Math|Transform|BreakTransform (Transformation|GetSocketTransform _sm_brick (Utilities|Array|Get(acopy) (Transformation|GetAllSocketNames _sm_brick) _array_index) "RTS_World"))) (.Rotation (Math|Transform|BreakTransform (Transformation|GetSocketTransform _sm_brick (Utilities|Array|Get(acopy) (Transformation|GetAllSocketNames _sm_brick) _array_index) "RTS_World")))) "Undefined" "MultiplyWithRoot" 0 (Utilities|Array|Get(acopy) _exitsthatareconnected _array_index) (Utilities|Array|Get(acopy) _encounters _array_index) self (Utilities|Array|Get(acopy) (Transformation|GetAllSocketNames _sm_brick) _array_index) 0))
      (Transformation|AttachActorToActor _returnvalue self (Utilities|Array|Get(acopy) (Transformation|GetAllSocketNames _sm_brick) _array_index) "KeepWorld" "KeepWorld" "KeepRelative" true)
      (Utilities|Array|Add (Variables|Default|GetExitObjs) _returnvalue))))

(fn InitWalls
  (Utilities|Array|Clear (Variables|Default|GetWalls))
  (for (_array_element _array_index) (.Exits (Utilities|Struct|BreakS_MapFragment (Variables|Default|GetMapFragmentInfo)))
    (Development|SetHiddeninGame (Utilities|Array|Get(acopy) (Utilities|Array|MakeArray (Variables|Default|GetSM_WallBlock0) (Variables|Default|GetSM_WallBlock1) (Variables|Default|GetSM_WallBlock2) (Variables|Default|GetSM_WallBlock3) (Variables|Default|GetSM_WallBlock4) (Variables|Default|GetSM_WallBlock5)) _array_index) _array_element false)
    (Collision|SetCollisionEnabled (Utilities|Array|Get(acopy) (Utilities|Array|MakeArray (Variables|Default|GetSM_WallBlock0) (Variables|Default|GetSM_WallBlock1) (Variables|Default|GetSM_WallBlock2) (Variables|Default|GetSM_WallBlock3) (Variables|Default|GetSM_WallBlock4) (Variables|Default|GetSM_WallBlock5)) _array_index) (select _array_element "NoCollision" "QueryAndPhysics"))
    (if (not _array_element)
      (Utilities|Array|Add (Variables|Default|GetWalls) (Utilities|Array|Get(acopy) (Utilities|Array|MakeArray (Variables|Default|GetSM_WallBlock0) (Variables|Default|GetSM_WallBlock1) (Variables|Default|GetSM_WallBlock2) (Variables|Default|GetSM_WallBlock3) (Variables|Default|GetSM_WallBlock4) (Variables|Default|GetSM_WallBlock5)) _array_index)))))

(fn ShowBuildingDecal
  (params (IsShown :type Boolean))
  (Rendering|SetVisibility (Variables|Default|GetDecal) IsShown false)
  (Variables|Default|SetIsGhost IsShown))

(fn SelectExit
  (params (ExitHit :type BP%20Exit%20Object%20Reference))
  (if (Variables|Default|GetIsGhost)
    (if (Utilities|Array|ContainsItem (Variables|Default|GetExitObjs) ExitHit)
      (if (== (Variables|Default|GetSelectedExit) ExitHit)
        _
        (else
          (Utilities|IsValid (Variables|Default|GetSelectedExit)
            (:Is%20Valid
              (Default|SetSelected (Variables|Default|GetSelectedExit) false))
            (:Is%20Not%20Valid
              _))
          (Variables|Default|SetSelectedExit ExitHit)
          (Default|SetSelected ExitHit true)
          (CallFunction|ShowBuildingDecal false)
          (return ExitHit))))
    (return (Variables|Default|GetSelectedExit))))

(fn CheckActorUnderCursor
  (bind _returnvalue (Game|GetPlayerController 0))
  (bind (_hitresult _returnvalue_2) (Game|Player|GetHitResultUnderCursorbyChannel _returnvalue "TraceTypeQuery1" true))
  (if _returnvalue_2
    (return (.HitActor (Collision|BreakHitResult _hitresult)))
    (else
      (return 0))))

(fn HighlightExit
  (if (Variables|Default|GetIsGhost)
    (bind _actorundercursor (CallFunction|CheckActorUnderCursor))
    (bind _asbp_exit (Utilities|Casting|CastToBP_Exit _actorundercursor)
      (:then
        (if (Utilities|Array|ContainsItem (Variables|Default|GetExitObjs) _asbp_exit)
          (if (== (Variables|Default|GetHighlightedExit) 0)
            (Default|SetHighlight _asbp_exit "NewEnumerator1")
            (Variables|Default|SetHighlightedExit _asbp_exit)
            (elif (not (== (Variables|Default|GetHighlightedExit) (Variables|Default|GetSelectedExit)))
              (if (not (== _asbp_exit (Variables|Default|GetSelectedExit)))
                (if (not (== (Variables|Default|GetHighlightedExit) _asbp_exit))
                  (Default|SetHighlight (Variables|Default|GetHighlightedExit) "NewEnumerator0")
                  (Default|SetHighlight _asbp_exit "NewEnumerator1")
                  (Variables|Default|SetHighlightedExit _asbp_exit)))))))
      (:CastFailed
        (Utilities|IsValid (Variables|Default|GetHighlightedExit)
          (:Is%20Valid
            (if (not (== (Variables|Default|GetSelectedExit) (Variables|Default|GetHighlightedExit)))
              (Default|SetHighlight (Variables|Default|GetHighlightedExit) "NewEnumerator0")
              (Variables|Default|SetHighlightedExit 0))))))))

(fn HighlightMoveField
  (bind _actorundercursor (CallFunction|CheckActorUnderCursor))
  (Utilities|Casting|CastToBP_MoveField _actorundercursor))

(fn FindUnConnectedExits
  (for _array_element (Variables|Default|GetExitObjs)
    (bind _outisconnected (Default|IsConnected _array_element))
    (if (not _outisconnected)
      (Utilities|Array|Add (LocalVariables|GetUnConnectedExits) _array_element)))
  (return (LocalVariables|GetUnConnectedExits)))

(fn SetCollsionEnableinExits
  (params (bNewActorEnableCollision :type Boolean))
  (for _array_element (Variables|Default|GetExitObjs)
    (Collision|SetActorEnableCollision _array_element bNewActorEnableCollision)))

(fn SetConnectedExits
  (params (ExitToConnect :type BP%20Exit%20Object%20Reference))
  (LocalVariables|SetNewExitsThatAreConnected (.ExitsThatAreConnected (Utilities|Struct|BreakS_MapFragment (Variables|Default|GetMapFragmentInfo))))
  (LocalVariables|SetIndexToFind (Utilities|Array|FindItem (Variables|Default|GetExitObjs) ExitToConnect))
  (bind (_array_element _array_index) (Utilities|Array|ForEachLoopwithBreak (.Exits (Utilities|Struct|BreakS_MapFragment (Variables|Default|GetMapFragmentInfo))) :!label _label)
    (:LoopBody
      (if _array_element
        (if (== (LocalVariables|Getcnt) (LocalVariables|GetIndexToFind))
          (Utilities|Array|SetArrayElem (LocalVariables|GetNewExitsThatAreConnected) _array_index true)
          (goto _label Break)
          (else
            (Math|Integer|IncrementInt (LocalVariables|Getcnt))))))
    (:Completed
      (Variables|Default|SetMapFragmentInfo (Utilities|Struct|MakeS_MapFragment (.IsStartingFragment (Utilities|Struct|BreakS_MapFragment (Variables|Default|GetMapFragmentInfo))) (.Exits (Utilities|Struct|BreakS_MapFragment (Variables|Default|GetMapFragmentInfo))) (LocalVariables|GetNewExitsThatAreConnected) (.Encounters (Utilities|Struct|BreakS_MapFragment (Variables|Default|GetMapFragmentInfo))) (.Transform (Utilities|Struct|BreakS_MapFragment (Variables|Default|GetMapFragmentInfo))))))))

(fn SetWallsVisible
  (params (IsVisible :type Boolean))
  (LocalVariables|SetWallsL (Utilities|Array|MakeArray (Variables|Default|GetSM_WallShort1) (Variables|Default|GetSM_WallShort) (Variables|Default|GetSM_WallLong1) (Variables|Default|GetSM_WallLong)))
  (for _array_element (Variables|Default|GetWalls)
    (Utilities|Array|Add (LocalVariables|GetWallsL) _array_element))
  (for _array_element_2 (LocalVariables|GetWallsL)
    (Development|SetHiddeninGame _array_element_2 (not IsVisible) false)
    (Collision|SetCollisionEnabled _array_element_2 (select IsVisible "QueryAndPhysics" "NoCollision"))))