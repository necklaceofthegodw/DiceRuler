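; Selectable map-generation object that shows default, highlighted or selected states on its static mesh.
; SetHighlight stores the state and writes a matching number to the HighlightColorNum scalar material parameter, leaving the visual to the material.
; SetSelected maps a boolean to the Selected or Default state through SetHighlight.
; BeginPlay caches the mesh's first material, though the highlight functions set the parameter through the mesh component.
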(event EventBeginPlay
  (Variables|Default|SetMeshMaterial (Rendering|Material|GetMaterial (Variables|Default|GetSM_Mesh) 0)))

(event Collision|EventActorBeginOverlap
  (params (OtherActor :type Actor%20Object%20Reference)))

(event EventTick
  (params (DeltaSeconds :type Float%20%28single-precision%29)))

(fn ConstructionScript)

(fn SetSelected
  (params (IsSelected :type Boolean))
  (CallFunction|SetHighlight (select IsSelected "NewEnumerator2" "NewEnumerator0")))

(fn SetHighlight
  (params (HighlightState :type E_HighlightState%20Enum :default "NewEnumerator0"))
  (bind _sm_mesh (Variables|Default|GetSM_Mesh))
  (bind _output_get (Variables|Default|SetHighlight%20State HighlightState))
  (switch Utilities|FlowControl|Switch|SwitchonE_HighlightState _output_get
    (:NewEnumerator0
      (Rendering|Material|SetScalarParameterValueonMaterials _sm_mesh "HighlightColorNum" 0.0))
    (:NewEnumerator1
      (Rendering|Material|SetScalarParameterValueonMaterials _sm_mesh "HighlightColorNum" 1.0))
    (:NewEnumerator2
      (Rendering|Material|SetScalarParameterValueonMaterials _sm_mesh "HighlightColorNum" 2.0))))