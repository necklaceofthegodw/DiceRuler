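; BP_RewardBasket is a basket actor that displays the rune fragments the player has collected.
; On BeginPlay it reads the collected fragment images from the DiceRuler game instance.
; It spawns one BP_RuneReward per image slightly above the basket mesh, passing the image at spawn and storing each actor in SpawnedRunes.
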(event EventBeginPlay
  (CallFunction|SpawnCollectedRunes))

(event Collision|EventActorBeginOverlap
  (params (OtherActor :type Actor%20Object%20Reference)))

(event EventTick
  (params (DeltaSeconds :type Float%20%28single-precision%29)))

(fn ConstructionScript)

(fn SpawnCollectedRunes
  (Utilities|Array|Clear (Variables|Default|GetSpawnedRunes))
  (bind _fragmentimages (Default|GetCollectedFragmentImages (CallFunction|GetDiceRulerGameInstance)))
  (for _array_element _fragmentimages
    (bind _returnvalue (Game|SpawnActorfromClass "/Game/DiceRuler/Puzzles/Memory/BP_RuneReward.BP_RuneReward_C" (Math|Transform|MakeTransform (+ (Transformation|GetWorldLocation (Variables|Default|GetSM_Basket)) "0.000000,0.000000,50.000000")) "Undefined" "MultiplyWithRoot" 0 _array_element 0))
    (Utilities|Array|Add (Variables|Default|GetSpawnedRunes) _returnvalue)))