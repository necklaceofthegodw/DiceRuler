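; Movement component for the top-down player controller that finds the move fields the pawn can step to, highlights the hovered one and moves the pawn.
; Every gameplay tick it enables map fragment exits, traces down for the current field, then traces four ways along the player's map fragment axes for available fields.
; An available field under the cursor gets highlighted, resetting the others.
; MoveTo uses SimpleMoveToLocation and spawns a cursor effect.
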(event EventBeginPlay
  (bind _asbp_top_down_controller (Utilities|Casting|CastToBP_TopDownController (Components|GetOwner)))
  (Variables|Default|SetBP_TopDownController _asbp_top_down_controller)
  (CallFunction|FindMoveFieldsinRange))

(event EventTick
  (params (DeltaSeconds :type Float%20%28single-precision%29))
  (switch Utilities|FlowControl|Switch|SwitchonE_InputMode (CallFunction|GetCurrentInputMode)
    (:NewEnumerator0
      (CallFunction|FindMoveFieldsinRange)
      (bind _actorundercursor (Default|CheckActorUnderCursor (Variables|Default|GetBP_TopDownController)))
      (bind _asbp_move_field (Utilities|Casting|CastToBP_MoveField _actorundercursor))
      (if (Utilities|Array|ContainsItem (Variables|Default|GetBP_MoveFieldsAvailable) _asbp_move_field)
        (for _array_element (Variables|Default|GetBP_MoveFieldsAvailable)
          (if (== _array_element _asbp_move_field)
            (Default|SetHighlight _asbp_move_field "NewEnumerator1")
            (else
              (Default|SetHighlight _array_element "NewEnumerator0"))))))))

(fn FindMoveFieldsinRange
  (bind _bp_topdowncontroller (Variables|Default|GetBP_TopDownController))
  (bind _returnvalue (Pawn|GetControlledPawn _bp_topdowncontroller))
  (Utilities|FlowControl|Sequence
    (:then_0
      (Default|EnableExitsinAllMapFragments (CallFunction|GetDiceMapFragmentManager) true)
      (Utilities|Array|Clear (Variables|Default|GetBP_MoveFieldsAvailable)))
    (:then_1
      (bind _outmapfragment (CallFunction|GetDicePlayerMapFragment))
      (bind _output_get (Variables|Default|SetPlayer%20Map%20Fragment _outmapfragment))
      (Utilities|IsValid _output_get
        (:Is%20Not%20Valid
          (return))))
    (:then_2
      (LocalVariables|SetTraceDirectionVectors (Utilities|Array|MakeArray (Transformation|GetActorRightVector (Variables|Default|GetPlayer%20Map%20Fragment)) (Math|Vector|NegateVector (Transformation|GetActorRightVector (Variables|Default|GetPlayer%20Map%20Fragment))) (Transformation|GetActorForwardVector (Variables|Default|GetPlayer%20Map%20Fragment)) (Math|Vector|NegateVector (Transformation|GetActorForwardVector (Variables|Default|GetPlayer%20Map%20Fragment)))))
      (bind _output_get_2 (LocalVariables|SetStartLocation (+ (Transformation|GetActorLocation _returnvalue) "0.000000,0.000000,-80.000000")))
      (bind _outhit (Collision|LineTraceByChannel _output_get_2 (+ _output_get_2 (* (Math|Vector|NegateVector (Transformation|GetActorUpVector _returnvalue)) 1e+02)) "TraceTypeQuery4" false 0 "None" true "(R=0.685470,G=0.021701,B=0.833333,A=1.000000)"))
      (bind _output_get_3 (LocalVariables|SetCurrentMoveField (.HitActor (Collision|BreakHitResult _outhit))))
      (bind _asbp_selectable_object (Utilities|Casting|CastToBP_SelectableObject _output_get_3))
      (switch Utilities|FlowControl|Switch|SwitchonE_HighlightState (Variables|/Game/DiceRuler/MapGeneration/Blueprints/BP_SelectableObject.BP_SelectableObject_C|GetHighlight%20State _asbp_selectable_object)
        (:NewEnumerator1
          _)
        (:NewEnumerator2
          _))
      (Default|SetHighlight _asbp_selectable_object "NewEnumerator0"))
    (:then_3
      (for _array_element (LocalVariables|GetTraceDirectionVectors)
        (bind _outhit_2 (Collision|LineTraceByChannel (LocalVariables|GetStartLocation) (+ (LocalVariables|GetStartLocation) (* _array_element (LocalVariables|GetTraceDistance))) "TraceTypeQuery4" false (Utilities|Array|MakeArray (LocalVariables|GetCurrentMoveField)) "None" true "(R=0.685470,G=0.021701,B=0.833333,A=1.000000)" "(R=0.000000,G=1.000000,B=0.000000,A=1.000000)" 2.0))
        (bind _asbp_move_field (Utilities|Casting|CastToBP_MoveField (.HitActor (Collision|BreakHitResult _outhit_2))))
        (Utilities|Array|Add (Variables|Default|GetBP_MoveFieldsAvailable) _asbp_move_field)))))

(fn Moveto
  (params (Location :type Vector))
  (AI|Navigation|SimpleMovetoLocation (.AsBP%20Top%20Down%20Controller (Utilities|Casting|CastToBP_TopDownController (Components|GetOwner))) Location)
  (Niagara|SpawnSystematLocation (Variables|Default|GetFXCursor) Location))