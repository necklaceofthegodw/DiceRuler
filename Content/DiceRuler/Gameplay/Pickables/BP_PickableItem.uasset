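; BP_PickableItem is a pickable item actor with an interaction trigger, a pickup widget and an empty OnInteract hook.
; Tick polls trigger overlap, claiming the player's ItemOverlapping slot and showing the widget only when no other item holds it.
; Tick also keeps the widget above the mesh along the player's up vector, facing the camera.
; Leaving the trigger clears the slot and hides the widget; DisableInteraction turns off trigger collision.
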(event OnComponentBeginOverlap(TriggerInteract)
  (params (OverlappedComponent :type Primitive%20Component%20Object%20Reference) (OtherActor :type Actor%20Object%20Reference) (OtherComp :type Primitive%20Component%20Object%20Reference) (OtherBodyIndex :type Integer) (bFromSweep :type Boolean) (SweepResult :type Hit%20Result%20Structure%20%28by%20ref%29)))

(event OnComponentEndOverlap(TriggerInteract)
  (params (OverlappedComponent :type Primitive%20Component%20Object%20Reference) (OtherActor :type Actor%20Object%20Reference) (OtherComp :type Primitive%20Component%20Object%20Reference) (OtherBodyIndex :type Integer))
  (bind _asbp_dice_player_character (Utilities|Casting|CastToBP_DicePlayerCharacter OtherActor))
  (Variables|/Game/DiceRuler/Player/BP_DicePlayerCharacter.BP_DicePlayerCharacter_C|SetItemOverlapping _asbp_dice_player_character 0)
  (CallFunction|ShowInteractionWidget false))

(event EventBeginPlay
  (bind _aswbp_pickup (Utilities|Casting|CastToWBP_Pickup (UserInterface|GetUserWidgetObject (Variables|Default|GetPickupWidgetComponent))))
  (Variables|Default|SetPickupWidget _aswbp_pickup))

(event Collision|EventActorBeginOverlap
  (params (OtherActor :type Actor%20Object%20Reference)))

(event EventTick
  (params (DeltaSeconds :type Float%20%28single-precision%29))
  (bind _dice_player_character (CallFunction|GetDicePlayerCharacter))
  (bind _pickupwidgetcomponent (Variables|Default|GetPickupWidgetComponent))
  (CallFunction|CheckIsOverlappingPlayer)
  ;[1 1 1] Rotate widget towards player
  (Utilities|IsValid _dice_player_character
    (:Is%20Valid
      (Transformation|SetWorldLocation _pickupwidgetcomponent (+ (Transformation|GetWorldLocation (Variables|Default|GetSM_Mesh)) (* (Transformation|GetActorUpVector _dice_player_character) 1.5e+02)) false false)
      (Transformation|SetWorldRotation _pickupwidgetcomponent (Math|Rotator|FindLookatRotation (Transformation|GetWorldLocation _pickupwidgetcomponent) (Camera|GetCameraLocation (Variables|/Script/Engine.PlayerController|GetPlayerCameraManager (CallFunction|GetDicePlayerController)))) false false))))

(fn ConstructionScript)

(fn ShowInteractionWidget
  (params (IsShown :type Boolean))
  (Utilities|IsValid (Variables|Default|GetPickupWidget)
    (:Is%20Valid
      (Development|SetHiddeninGame (Variables|Default|GetPickupWidgetComponent) (not IsShown) false))))

(fn OnInteract)

(fn DisableInteraction
  (Collision|SetCollisionEnabled (Variables|Default|GetTriggerInteract) "NoCollision"))

(fn CheckIsOverlappingPlayer
  (bind _dice_player_character (CallFunction|GetDicePlayerCharacter))
  (if (Collision|IsOverlappingActor (Variables|Default|GetTriggerInteract) _dice_player_character :!class /Script/Engine.PrimitiveComponent)
    (if (not (== (Variables|/Game/DiceRuler/Player/BP_DicePlayerCharacter.BP_DicePlayerCharacter_C|GetItemOverlapping _dice_player_character) self))
      (CallFunction|ShowInteractionWidget (not (Utilities|IsValid (Variables|/Game/DiceRuler/Player/BP_DicePlayerCharacter.BP_DicePlayerCharacter_C|GetItemOverlapping _dice_player_character))))
      (if (not (Utilities|IsValid (Variables|/Game/DiceRuler/Player/BP_DicePlayerCharacter.BP_DicePlayerCharacter_C|GetItemOverlapping _dice_player_character)))
        (Variables|/Game/DiceRuler/Player/BP_DicePlayerCharacter.BP_DicePlayerCharacter_C|SetItemOverlapping _dice_player_character self)))))