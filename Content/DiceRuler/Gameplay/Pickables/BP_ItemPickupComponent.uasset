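; Actor component for the dice player character that lets it pick up and drop physical items.
; Picking up removes the overlapping item from any balance scale, hides its interaction widget and disables its physics and collision.
; A timeline added at runtime on BeginPlay lerps the item toward the mesh's WeaponSocket, then attaches it there.
; Dropping detaches the held item and restores physics and collision.
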(event Custom|TryPickingUpItem
  (bind _itemoverlapping (Variables|Default|GetItemOverlapping))
  (bind _balancescale (Variables|/Game/DiceRuler/Gameplay/Pickables/BP_PickableItem.BP_PickableItem_C|GetBalanceScale _itemoverlapping))
  (if (not (Variables|Default|GetIsPickingUp))
    (if (not (== (Variables|Default|GetItemOverlapping) (Variables|Default|GetPickedItem)))
      (Utilities|IsValid (Variables|Default|GetPickedItem)
        (:Is%20Not%20Valid
          (Utilities|IsValid (Variables|Default|GetItemOverlapping)
            (:Is%20Valid
              ;[1 1 1] TODO add event on item picked, that the balance scale will listen to and update sockets occupied by pickables
              (Utilities|IsValid _balancescale
                (:Is%20Valid
                  (Default|RemoveItemfromSocket _balancescale _itemoverlapping))
                (:Is%20Not%20Valid
                  _))
              (Variables|Default|SetPickedItem (Variables|Default|GetItemOverlapping))
              (Variables|Default|SetIsPickingUp true)
              (Default|ShowInteractionWidget (Variables|Default|GetPickedItem) false)
              (Physics|SetSimulatePhysics (Variables|/Game/DiceRuler/Gameplay/Pickables/BP_PickableItem.BP_PickableItem_C|GetSM_Mesh (Variables|Default|GetPickedItem)) false)
              (Collision|SetCollisionEnabled (Variables|/Game/DiceRuler/Gameplay/Pickables/BP_PickableItem.BP_PickableItem_C|GetSM_Mesh (Variables|Default|GetPickedItem)) "NoCollision")
              (Components|Timeline|PlayfromStart (Variables|Default|GetPickupTimeline)))))))))

(event Custom|TryDroppingItem
  (if (not (Variables|Default|GetIsPickingUp))
    (Utilities|IsValid (Variables|Default|GetPickedItem)
      (:Is%20Valid
        (Transformation|DetachFromActor (Variables|Default|GetPickedItem) "KeepWorld" "KeepWorld" "KeepWorld")
        (Collision|SetCollisionEnabled (Variables|/Game/DiceRuler/Gameplay/Pickables/BP_PickableItem.BP_PickableItem_C|GetSM_Mesh (Variables|Default|GetPickedItem)) "QueryAndPhysics")
        (Physics|SetSimulatePhysics (Variables|/Game/DiceRuler/Gameplay/Pickables/BP_PickableItem.BP_PickableItem_C|GetSM_Mesh (Variables|Default|GetPickedItem)) true)
        (Variables|Default|SetPickedItem 0)))))

(event Custom|UpdatePickingUp
  (params (time :type Float%20%28single-precision%29))
  (bind _pickeditem (Variables|Default|GetPickedItem))
  (Utilities|IsValid _pickeditem
    (:Is%20Valid
      (Transformation|SetActorLocation _pickeditem (Math|Vector|Lerp(Vector) (Transformation|GetActorLocation (Variables|Default|GetPickedItem)) (Transformation|GetSocketLocation (Variables|/Script/Engine.Character|GetMesh (Variables|Default|GetParentDiceCharacter)) "WeaponSocket") time) false false))
    (:Is%20Not%20Valid
      (Variables|Default|SetIsPickingUp false))))

(event Custom|FinishedPickingUp
  (bind _pickeditem (Variables|Default|GetPickedItem))
  (Utilities|IsValid _pickeditem
    (:Is%20Valid
      (Transformation|AttachComponentToComponent _pickeditem (Variables|/Script/Engine.Character|GetMesh (Variables|Default|GetParentDiceCharacter)) "WeaponSocket" "SnapToTarget" "SnapToTarget" "KeepRelative" true))
    (:Is%20Not%20Valid
      _))
  (Variables|Default|SetIsPickingUp false))

(event EventBeginPlay
  (bind _output_get (Variables|Default|SetParentDiceCharacter (.AsBP%20Dice%20Player%20Character (Utilities|Casting|CastToBP_DicePlayerCharacter (Components|GetOwner)))))
  (bind _returnvalue (Game|AddComponentbyClass _output_get "/Script/Engine.TimelineComponent"))
  (Class|TimelineComponent|AddInterpFloat _returnvalue (Variables|Default|GetFloat%20Curve) (EventDispatchers|CreateEvent :!event UpdatePickingup) "None" "None")
  (Class|TimelineComponent|SetTimelineFinishedFunc _returnvalue (EventDispatchers|CreateEvent :!event Custom|FinishedPickingUp))
  (Variables|Default|SetPickupTimeline _returnvalue))

(event EventTick
  (params (DeltaSeconds :type Float%20%28single-precision%29)))