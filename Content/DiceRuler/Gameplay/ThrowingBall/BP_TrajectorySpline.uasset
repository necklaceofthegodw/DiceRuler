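; Trajectory spline actor for the ball-throwing gameplay, drawing a path through supplied points as a dashed line.
; SetupSpline clears and rebuilds the spline from the rebased points, adding one spline mesh per point.
; A FlipFlop alternates red and transparent materials to create the dashes, then each mesh is bent between consecutive spline points using their tangents.
; Existing spline meshes are never cleared, and all other graphs are empty.
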(event EventBeginPlay)

(event Collision|EventActorBeginOverlap
  (params (OtherActor :type Actor%20Object%20Reference)))

(event EventTick
  (params (DeltaSeconds :type Float%20%28single-precision%29)))

(fn ConstructionScript)

(fn SetupSpline
  (params (SplinePoints :type Array%20of%20Vectors))
  (bind _spline (Variables|Default|GetSpline))
  (bind _spline_2 (Variables|Default|GetSpline))
  (Spline|ClearSplinePoints _spline true)
  (for _array_element SplinePoints
    (Spline|AddSplinePoint _spline (Class|GameplayStatics|RebaseZeroOriginOntoLocal _array_element) "Local" true)
    (Utilities|FlowControl|FlipFlop
      (:A
        (bind _returnvalue (AddComponent|AddSplineMeshComponent true))
        (Rendering|Material|SetMaterial _returnvalue 0 "/Engine/EngineDebugMaterials/VertexColorViewMode_RedOnly.VertexColorViewMode_RedOnly")
        (Utilities|Array|Add (Variables|Default|GetSplineMeshes) _returnvalue))
      (:B
        (bind _returnvalue_2 (AddComponent|AddSplineMeshComponent true))
        (Rendering|Material|SetMaterial _returnvalue_2 0 "/Game/DiceRuler/Gameplay/ThrowingBall/M_Transparent.M_Transparent")
        (Utilities|Array|Add (Variables|Default|GetSplineMeshes) _returnvalue_2))))
  (for (_array_element_2 _array_index) (Variables|Default|GetSplineMeshes)
    (SplineMesh|SetStartandEnd _array_element_2 (.Location (Spline|GetLocationandTangentatSplinePoint _spline_2 _array_index "Local")) (.Tangent (Spline|GetLocationandTangentatSplinePoint _spline_2 _array_index "Local")) (.Location (Spline|GetLocationandTangentatSplinePoint _spline_2 (+ _array_index 1) "Local")) (.Tangent (Spline|GetLocationandTangentatSplinePoint _spline_2 (+ _array_index 1) "Local")) true :!class /Script/Engine.SplineMeshComponent)))